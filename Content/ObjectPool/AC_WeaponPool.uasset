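; Weapon pool component that pre-spawns weapon actors so they can be reused.
; On BeginPlay it spawns one actor per pooled class, marked not in use, but only prints a warning if over three classes are set.
; SpawnFromPool sets the indexed weapon's transform, marks it in use and returns it.
; Its FirstAvailableActor result goes unused, and the in-use check runs only for index -1.
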(event `self.ReceiveBeginPlay`
  (`self.InitializePool`))

(event `InitializePool`
  (if (> (`KismetArrayLibrary.Array_Length` (`self.PooledActorClass`)) 3)
    (`KismetSystemLibrary.PrintString` "A lot of weapons")
    (else
      (for _array_element (`self.PooledActorClass`)
        (bind _returnvalue (`|SpawnActorFromClass` _array_element (`KismetMathLibrary.MakeTransform` (0.0 0.0 0.0)) "Undefined" "MultiplyWithRoot" (`self.GetOwner`) null))
        (`KismetArrayLibrary.Array_AddUnique` (`self.WeaponPool`) _returnvalue)
        (`/Game/ObjectPool/BP_PooledActor.SetInUse` _returnvalue false)))))

(fn `FirstAvailableActor`
  (returns (PooledWeapon :type "/Game/Weapons/default/parentBP/BP_WeaponBase Object Reference"))
  (for _array_element (`self.WeaponPool`)
    (if (not (`/Game/ObjectPool/BP_PooledActor.InUse` _array_element))
      (return _array_element))))

(fn `SpawnFromPool`
  (params (WeaponIndex :type Integer))
  (returns (PooledWeapon :type "/Game/Weapons/default/parentBP/BP_WeaponBase Object Reference"))
  (bind _output (`|GetArrayItem` (`self.WeaponPool`) WeaponIndex))
  (if (!= WeaponIndex -1)
    (`self.FirstAvailableActor`)
    (`/Engine/EditorBlueprintResources/StandardMacros.IsValid` _output :!label _label
      (:`Is Valid`
        _)
      (:`Is Not Valid`
        (`KismetSystemLibrary.PrintString` "Invalid weapon pool element")
        (return null)))
    (elif (not (`/Game/ObjectPool/BP_PooledActor.InUse` _output))
      (goto _label)
      (else
        (`KismetSystemLibrary.PrintString` "Selected Weapon is still in use")
        (return null))))
  (`Actor.K2_SetActorTransform` _output (`KismetMathLibrary.MakeTransform` (0.0 0.0 0.0)) false false)
  (`/Game/ObjectPool/BP_PooledActor.SetInUse` _output true)
  (return _output))