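; Base weapon Blueprint that handles equip, stow and projectile firing through WeaponComponent delegates.
; Equip and stow notify the wielder; stowing clears in-use, while setting in-use attaches the weapon to the owning pawn.
; Firing spawns CustomProjectile at the muzzle aimed at the hit or trace end, and the wielder ignores it when moving.
; Projectile impact spawns an optional AOE actor; DeployProjectileFiredFX is an empty hook called on fire.
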(event `self.WeaponComponent.OnStowDelegate`
  (params (WeaponWielder :type "Actor Object Reference") (Weapon :type "TP_WeaponComponent Object Reference"))
  (message `WeaponWielderInterface.OnStow` WeaponWielder)
  (`self.SetInUse` false))

(event `self.WeaponComponent.OnEquipDelegate`
  (params (WeaponWielder :type "Actor Object Reference") (Weapon :type "TP_WeaponComponent Object Reference"))
  (message `WeaponWielderInterface.OnEquip` WeaponWielder))

(event `self.SetInUse`
  (params (InUse :type Boolean))
  (`parent.SetInUse` InUse)
  (if InUse
    (bind _aspawn (cast `Pawn` (`self.GetOwner`)))
    (message `WeaponWielderInterface.AttachWeapon` _aspawn (`self.WeaponComponent`))))

(event `self.WeaponComponent.OnWeaponProjectileFireDelegate`
  (params (HitResult :type "HitResult Structure"))
  (bind (_bblockinghit _binitialoverlap _time _distance _location _impactpoint _normal _impactnormal _physmat _hitactor _hitcomponent _hitbonename _bonename _hititem _elementindex _faceindex _tracestart _traceend) (`GameplayStatics.BreakHitResult` HitResult))
  (bind _returnvalue (`SceneComponent.GetSocketLocation` (`self.WeaponComponent`) (`self.MuzzleSocket`)))
  (bind _returnvalue_2 (`TP_WeaponComponent.GetOwningWeaponWielder` (`self.WeaponComponent`)))
  (`self.DeployProjectileFiredFX` HitResult)
  (bind _returnvalue_3 (`|SpawnActorFromClass` (`self.CustomProjectile`) (`KismetMathLibrary.MakeTransform` _returnvalue (`KismetMathLibrary.FindLookAtRotation` _returnvalue (select `bool` _bblockinghit :`false` _traceend :`true` _location))) "Undefined" "MultiplyWithRoot" _returnvalue_2 10000.0 0.0 false 2000.0 false null _returnvalue_2))
  (bind _asprimitive_component (cast `PrimitiveComponent` (`Actor.RootComponent` (`TP_WeaponComponent.GetOwningWeaponWielder` (`self.WeaponComponent`)))))
  (`PrimitiveComponent.IgnoreActorWhenMoving` _asprimitive_component _returnvalue_3 true)
  (add `CustomProjectile.OnProjectileImpactDelegate` _returnvalue_3 (delegate `ProjectileImpact`)))

(event `ProjectileImpact`
  (params (OtherActor :type "Actor Object Reference") (Hit :type "HitResult Structure"))
  (bind _aoeclass (`self.AOEClass`))
  (if (`KismetSystemLibrary.IsValidClass` _aoeclass)
    (`|SpawnActorFromClass` _aoeclass (`KismetMathLibrary.MakeTransform` (`.Location` (`GameplayStatics.BreakHitResult` Hit))) "Undefined" "MultiplyWithRoot" null (`TP_WeaponComponent.GetOwningWeaponWielder` (`self.WeaponComponent`)))))

(fn `DeployProjectileFiredFX`
  (params (`Hit Result` :type "HitResult Structure")))

(fn `UserConstructionScript`
  (`parent.UserConstructionScript`))