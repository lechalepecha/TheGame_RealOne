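; Base enemy character that chases and melee-kicks the player, handles weapon equip state, and plays hit, stagger, stun, knockback and death reactions.
; Health, damage and attack tokens route through BPCDamageSystem, whose death and damage events are bound at BeginPlay.
; Attacks reserve tokens from the target, return them when finished, and land via a notify-driven sphere trace.
; Death stops AI, launches a ragdoll, then decrements the enemy manager's count.
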(event `self.ReceiveBeginPlay`
  (bind _bpc_damagesystem (`self.BPC_DamageSystem`))
  (bind _asaic_enemy_base (cast `/Game/Enemies/AI/AIC_Enemy_Base` (`AIBlueprintHelperLibrary.GetAIController` self)))
  (set `self.AIC Enemy Base` _asaic_enemy_base)
  (add `/Game/DamageSystem/AC_DamageSystem.OnDeath` _bpc_damagesystem (`|CreateDelegate` :!event `Die`))
  (add `/Game/DamageSystem/AC_DamageSystem.OnDamageResponce` _bpc_damagesystem (`|CreateDelegate` :!event `RespondDamage`))
  (`SkeletalMeshComponent.LinkAnimClassLayers` (`self.Mesh`) "/Game/Characters/Mannequins/Animations/ABP_RangedEnemy.ABP_RangedEnemy_C")
  (`/Engine/EditorBlueprintResources/StandardMacros.IsValid` (`self.EnemyManager`)
    (:`Is Not Valid`
      (bind _outactors (`GameplayStatics.GetAllActorsOfClass` "/Game/Enemies/BP_Enemy_Manager.BP_Enemy_Manager_C"))
      (for _array_element _outactors
        (set `self.EnemyManager` _array_element)))))

(event `self.ReceiveTick`
  (params (DeltaSeconds :type "Float (single-precision)"))
  (bind _returnvalue (`GameplayStatics.GetPlayerCharacter` 0))
  (bind _bodyrotationcyl (`self.BodyRotationCyl`))
  (bind (_returnvalue_roll _returnvalue_pitch) (`KismetMathLibrary.BreakRotator` (`KismetMathLibrary.FindLookAtRotation` (`SceneComponent.K2_GetComponentLocation` _bodyrotationcyl) (`self.K2_GetActorLocation` _returnvalue))))
  (bind _asbp_fpcharacter (cast `/Game/FirstPerson/Blueprints/BP_FPCharacter` _returnvalue))
  (bind _output_get (set `self.Player` _asbp_fpcharacter))
  (set `self.LookAtLocation` (`SceneComponent.GetSocketLocation` (`MainCharacter.GetMesh1P` _output_get) "spine_05"))
  (`SceneComponent.K2_SetWorldRotation` _bodyrotationcyl (`KismetMathLibrary.MakeRotator` _returnvalue_pitch) false false)
  (set `self.BodyRotation` (* _returnvalue_pitch -1.0)))

(event `Chase Player`
  (bind _returnvalue (`GameplayStatics.GetPlayerCharacter` 0))
  (`|AIMoveTo` self (0.0 0.0 0.0) _returnvalue 100.0
    (:`OnSuccess`
      (`/Game/Enemies/AI/BPI_EnemyAI.MeleeAttack` self _returnvalue)
      (`KismetSystemLibrary.Delay` 2.0)
      (`self.Chase Player`))))

(event `/Game/Enemies/AI/BPI_EnemyAI.MeleeAttack`
  (params (AttackTarget :type "Actor Object Reference"))
  (bind _notifyname (`|PlayMontage` (`self.Mesh`) (`KismetArrayLibrary.Array_Random` (`|MakeArray` "/Game/Characters/Heroes/Mannequin/Animations/Locomotion/Unarmed/AM_MM_Unarmed_Attack_StandingMeleeKick.AM_MM_Unarmed_Attack_StandingMeleeKick" :!type "AnimMontage Object Reference")))
    (:`then`
      (set `/Game/DamageSystem/AC_DamageSystem.IsInterruptable` false (`self.BPC_DamageSystem`)))
    (:`OnCompleted`
      (`self.AttackEnd` AttackTarget :!label _label)
      (set `/Game/DamageSystem/AC_DamageSystem.IsInterruptable` true (`self.BPC_DamageSystem`)))
    (:`OnInterrupted`
      (goto _label))
    (:`OnNotifyBegin`
      (if (== _notifyname "Melee")
        (`self.SphereTraceMelee`)))))

(event `/Game/Enemies/AI/BPI_EnemyAI.ForceStopAttacking`
  (`self.On Attack End`))

(event `Die`
  (bind _mesh (`self.Mesh`))
  (`/Game/Enemies/AI/BPI_EnemyAI.ForceStopAttacking`)
  (`BrainComponent.StopLogic` (`AIController.BrainComponent` (`self.AIC Enemy Base`)) "")
  (`PrimitiveComponent.SetCollisionResponseToChannel` _mesh "ECC_Pawn" "ECR_Overlap")
  (`MovementComponent.StopMovementImmediately` (`self.CharacterMovement`))
  (`|PlayMontage` (`self.Mesh`) (`KismetArrayLibrary.Array_Random` (`|MakeArray` "/Game/Characters/Heroes/Mannequin/Animations/Actions/AM_MM_Death_Back_01.AM_MM_Death_Back_01" "/Game/Characters/Heroes/Mannequin/Animations/Actions/AM_MM_Death_Front_01.AM_MM_Death_Front_01" "/Game/Characters/Heroes/Mannequin/Animations/Actions/AM_MM_Death_Front_02.AM_MM_Death_Front_02" "/Game/Characters/Heroes/Mannequin/Animations/Actions/AM_MM_Death_Front_03.AM_MM_Death_Front_03" "/Game/Characters/Heroes/Mannequin/Animations/Actions/AM_MM_Death_Left_01.AM_MM_Death_Left_01" "/Game/Characters/Heroes/Mannequin/Animations/Actions/AM_MM_Death_Right_01.AM_MM_Death_Right_01" :!type "AnimMontage Object Reference"))
    (:`then`
      (`self.LaunchCharacter` self (* (`KismetMathLibrary.Normal` (- (`self.K2_GetActorLocation`) (`self.LastKnockBack`))) 15000.0) true true)
      (`PrimitiveComponent.SetSimulatePhysics` (`self.Mesh`) true)
      (`PrimitiveComponent.SetCollisionEnabled` _mesh "QueryAndPhysics")
      (`PrimitiveComponent.SetCollisionEnabled` (`self.CapsuleComponent`) "NoCollision")
      (`KismetSystemLibrary.Delay` 3.0)
      (`self.K2_DestroyActor`)
      (`/Engine/EditorBlueprintResources/StandardMacros.DecrementInt` (`/Game/Enemies/BP_Enemy_Manager.EnemyCount` (`self.EnemyManager`))))))

(event `RespondDamage`
  (params (DamageResponce :type "/Game/DamageSystem/Enum/E_DamageResponce Enum" :default "NewEnumerator0") (DamageCuaser :type "Actor Object Reference") (KnockbackEpicenter :type "Vector Structure") (HitBoneName :type Name) (DamageDirection :type "/Game/DamageSystem/Enum/E_DamageDirection Enum" :default "NewEnumerator0"))
  (bind _returnvalue (`KismetMathLibrary.RandomIntegerInRange` 0 1))
  (bind _output_get (set `self.LastKnockBack` KnockbackEpicenter))
  (switch `/Game/DamageSystem/Enum/E_DamageResponce` DamageResponce
    (:`NewEnumerator1`
      (`|PlayMontage` (`self.Mesh`) (select `/Game/DamageSystem/Enum/E_DamageDirection` DamageDirection :`NewEnumerator1` (select `int` (`KismetMathLibrary.RandomIntegerInRange` 0 3) :`0` "/Game/Characters/Heroes/Mannequin/Animations/Actions/AM_MM_HitReact_Front_Hvy_01.AM_MM_HitReact_Front_Hvy_01" :`1` "/Game/Characters/Heroes/Mannequin/Animations/Actions/AM_MM_HitReact_Front_Lgt_01.AM_MM_HitReact_Front_Lgt_01" :`2` "/Game/Characters/Heroes/Mannequin/Animations/Actions/AM_MM_HitReact_Front_Med_01.AM_MM_HitReact_Front_Med_01" :`3` "/Game/Characters/Heroes/Mannequin/Animations/Actions/AM_MM_HitReact_Front_Med_02.AM_MM_HitReact_Front_Med_02" :!type "AnimMontage Object Reference") :`NewEnumerator2` (select `int` (`KismetMathLibrary.RandomIntegerInRange` 0 1) :`0` "/Game/Characters/Heroes/Mannequin/Animations/Actions/AM_MM_HitReact_Back_Lgt_01.AM_MM_HitReact_Back_Lgt_01" :`1` "/Game/Characters/Heroes/Mannequin/Animations/Actions/AM_MM_HitReact_Back_Med_01.AM_MM_HitReact_Back_Med_01" :!type "AnimMontage Object Reference") :`NewEnumerator3` (select `int` _returnvalue :`0` "/Game/Characters/Heroes/Mannequin/Animations/Actions/AM_MM_HitReact_Left_Lgt_01.AM_MM_HitReact_Left_Lgt_01" :`1` "/Game/Characters/Heroes/Mannequin/Animations/Actions/AM_MM_HitReact_Left_Med_01.AM_MM_HitReact_Left_Med_01" :!type "AnimMontage Object Reference") :`NewEnumerator4` (select `int` _returnvalue :`0` "/Game/Characters/Heroes/Mannequin/Animations/Actions/AM_MM_HitReact_Right_Lgt_01.AM_MM_HitReact_Right_Lgt_01" :`1` "/Game/Characters/Heroes/Mannequin/Animations/Actions/AM_MM_HitReact_Right_Med_01.AM_MM_HitReact_Right_Med_01" :!type "AnimMontage Object Reference"))))
    (:`NewEnumerator2`
      (`MovementComponent.StopMovementImmediately` (`self.CharacterMovement`))
      (`|PlayMontage` (`self.Mesh`) (select `int` (`KismetMathLibrary.RandomIntegerInRange` 0 2) :`0` "/Game/Characters/Heroes/Mannequin/Animations/Actions/MM_Staggered_Front_01_Montage.MM_Staggered_Front_01_Montage" :`1` "/Game/Characters/Heroes/Mannequin/Animations/Actions/MM_Staggered_Front_02_Montage.MM_Staggered_Front_02_Montage" :`2` "/Game/Characters/Heroes/Mannequin/Animations/Actions/MM_Staggered_Front_03_Montage.MM_Staggered_Front_03_Montage" :!type "AnimMontage Object Reference")
        (:`then`
          _)
        (:`OnCompleted`
          _)
        (:`OnInterrupted`
          _))
      (bind _aic_enemy_base (`self.AIC Enemy Base`)
        (:`then`
          (`/Game/Enemies/AI/AIC_Enemy_Base.SetStateAsFrozen` _aic_enemy_base))
        (:`else`)))
    (:`NewEnumerator3`
      (set `self.CustomTimeDilation` 0.05)
      (`KismetSystemLibrary.PrintString` "stuned ")
      (`KismetSystemLibrary.Delay` 5.0)
      (set `self.CustomTimeDilation` 1.0))
    (:`NewEnumerator4`
      (`|PlayMontage` (`self.Mesh`) "/Game/Characters/Heroes/Mannequin/Animations/Actions/AM_MM_HitReact_Front_Hvy_01.AM_MM_HitReact_Front_Hvy_01"
        (:`then`
          (bind (_returnvalue_x _returnvalue_y) (`KismetMathLibrary.BreakVector` (* (`KismetMathLibrary.Normal` (- _output_get (`self.K2_GetActorLocation`))) -1500.0)))
          (`self.LaunchCharacter` self (`KismetMathLibrary.MakeVector` _returnvalue_x _returnvalue_y) true true))))))

(event `/Game/Enemies/AI/BPI_EnemyAI.EquipWeapon`
  (`|PlayMontage` (`self.Mesh`)
    (:`OnCompleted`
      _)
    (:`OnInterrupted`
      _))
  (set `self.IsWeaponEquiped` true)
  (`self.OnWeaponEquipped`))

(event `/Game/Enemies/AI/BPI_EnemyAI.UnequipWeapon`
  (set `self.IsWeaponEquiped` false)
  (`SkeletalMeshComponent.LinkAnimClassLayers` (`self.Mesh`) "/Game/Characters/Heroes/Mannequin/Animations/Locomotion/Unarmed/ABP_UnarmedAnimLayers.ABP_UnarmedAnimLayers_C"))

(event `/Game/DamageSystem/BPI_Damagable.ReturnAttackToken`
  (params (Amount :type Integer))
  (`/Game/DamageSystem/AC_DamageSystem.ReturnAttackToken` (`self.BPC_DamageSystem`) Amount))

(event `/Game/Enemies/AI/BPI_EnemyAI.StoreAttackTokens`
  (params (AttackTarget :type "Actor Object Reference") (TokensAmount :type Integer))
  (bind (_value _returnvalue) (`BlueprintMapLibrary.Map_Find` (`self.ReservedAttackTokens`) AttackTarget))
  (`BlueprintMapLibrary.Map_Add` (`self.ReservedAttackTokens`) AttackTarget (`KismetMathLibrary.SelectInt` (+ TokensAmount _value) TokensAmount _returnvalue)))

(event `/Game/Enemies/AI/BPI_EnemyAI.AttackEnd`
  (params (AttackTarget :type "Actor Object Reference"))
  (bind _tokensused (`self.TokensUsed`))
  (message `/Game/DamageSystem/BPI_Damagable.ReturnAttackToken` AttackTarget _tokensused)
  (`/Game/Enemies/AI/BPI_EnemyAI.StoreAttackTokens` AttackTarget (* _tokensused -1))
  (`self.On Attack End`))

(fn `GetCurrentHealth`
  (returns (Health :type "Float (double-precision)"))
  (return (`/Game/DamageSystem/AC_DamageSystem.Health` (`self.BPC_DamageSystem`))))

(fn `GetFocusPoint`
  (returns (FocusActor :type "Actor Object Reference"))
  (return null))

(fn `GetIdealRange`
  (returns (AttackRadius :type "Float (double-precision)") (DefendRadius :type "Float (double-precision)"))
  (return 225.0 350.0))

(fn `GetMaxHealth`
  (returns (MaxHealth :type "Float (double-precision)"))
  (return (`/Game/DamageSystem/AC_DamageSystem.MaxHealth` (`self.BPC_DamageSystem`))))

(fn `GetPatrolRoute`
  (returns (PatrolRoute :type "/Game/Enemies/AI/Routes/BP_PatrolRoute Object Reference"))
  (return (`self.PatrolRoute`)))

(fn `Heal`
  (params (Ammount :type "Float (double-precision)"))
  (returns (NewHealth :type "Float (double-precision)"))
  (bind _newhealth (`/Game/DamageSystem/AC_DamageSystem.Heal` (`self.BPC_DamageSystem`) Ammount))
  (return _newhealth))

(fn `IsDead`
  (returns (IsDead :type Boolean))
  (return (`/Game/DamageSystem/AC_DamageSystem.IsDead` (`self.BPC_DamageSystem`))))

(fn `ReserveAttackToken`
  (params (Amount :type Integer))
  (returns (Success :type Boolean))
  (bind _success (`/Game/DamageSystem/AC_DamageSystem.ReservAttackToken` (`self.BPC_DamageSystem`) Amount))
  (return _success))

(fn `SphereTraceMelee`
  (returns (`Return Value` :type Boolean))
  (bind _returnvalue (`self.K2_GetActorLocation`))
  (bind _instigator (`self.Instigator`))
  (bind (_outhit _returnvalue_2) (`KismetSystemLibrary.SphereTraceSingleForObjects` _returnvalue (+ _returnvalue (* (`self.GetActorForwardVector`) 225.0)) 20.0 (`|MakeArray` "ObjectTypeQuery3" :!type "EObjectTypeQuery Enum") false (`|MakeArray` self :!type "Actor Object Reference") "None" true (struct :`R` 1.0 :`A` 1.0) (struct :`G` 1.0 :`A` 1.0) 2.0))
  (if _returnvalue_2
    (bind (_bblockinghit _binitialoverlap _time _distance _location _impactpoint _normal _impactnormal _physmat _hitactor _hitcomponent _hitbonename) (`GameplayStatics.BreakHitResult` _outhit))
    (bind (_wasdamaged _wasdamagedtodeath _finaldamage) (message `/Game/DamageSystem/BPI_Damagable.TakeDamage` _hitactor (make `/Game/DamageSystem/Struct/S_DamageInfo` 30.0 "NewEnumerator1" "NewEnumerator4" false false true false _location _normal _hitbonename 1.0) _instigator (0.0 0.0 0.0)))
    (`GameplayStatics.SpawnSoundAtLocation` null _location (struct) 1.0 1.0 0.0 null null)
    (`AISense_Damage.ReportDamageEvent` _hitactor _instigator _finaldamage (`self.K2_GetActorLocation`))
    (return false)))

(fn `StartAttack`
  (params (AttackTarget :type "Actor Object Reference") (TokensNeeded :type Integer))
  (returns (Success :type Boolean))
  (bind _success (message `/Game/DamageSystem/BPI_Damagable.ReserveAttackToken` AttackTarget TokensNeeded))
  (if _success
    (`/Game/Enemies/AI/BPI_EnemyAI.StoreAttackTokens` AttackTarget TokensNeeded)
    (set `self.TokensUsed` TokensNeeded)
    (return true)
    (else
      (return false))))

(fn `TakeDamage`
  (params (DamageInfo :type "/Game/DamageSystem/Struct/S_DamageInfo Structure") (DamageCauser :type "Actor Object Reference") (`Knockback Epicenter` :type "Vector Structure"))
  (returns (WasDamaged :type Boolean) (WasDamagedToDeath :type Boolean) (FinalDamage :type "Float (double-precision)") (IsCriticalHit :type Boolean))
  (bind (_wasdamaged _wasdamagedtodeath _finaldamage _iscriticalhit) (`/Game/DamageSystem/AC_DamageSystem.TakeDamage` (`self.BPC_DamageSystem`) DamageInfo DamageCauser `Knockback Epicenter`))
  (if _wasdamaged
    (return _wasdamaged _wasdamagedtodeath _finaldamage _iscriticalhit)))

(fn `UpdateMovementSpeed`
  (params (SpeedType :type "/Game/Enemies/AI/Enums/E_MovementSpeed Enum" :default "NewEnumerator0"))
  (returns (`Speed Value` :type "Float (double-precision)"))
  (bind _output_get (set `CharacterMovementComponent.MaxWalkSpeed` (select `/Game/Enemies/AI/Enums/E_MovementSpeed` SpeedType :`NewEnumerator1` 175.0 :`NewEnumerator2` 350.0 :`NewEnumerator3` 500.0) (`self.CharacterMovement`)))
  (return _output_get))

(fn `UpdateState`
  (params (NewState :type "/Game/Enemies/AI/Enums/E_EnemyStates Enum" :default "NewEnumerator0"))
  (returns (State :type "/Game/Enemies/AI/Enums/E_EnemyStates Enum"))
  (return NewState))

(fn `UserConstructionScript`)