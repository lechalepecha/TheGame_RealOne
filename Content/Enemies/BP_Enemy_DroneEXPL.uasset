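; Exploding drone enemy that damages the player after they come within range of its trigger sphere.
; CallCalctheRoute asks DroneBounds to compute a route from the drone to the player's current location.
; Player overlap starts a Timeline as a fuse, then plays an explosion sound, sends damage and calls Die.
; Leaving the sphere does not cancel the fuse, so damage still applies.
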(event `self.CallCalcTheRoute`
  (message `FlyingNavigationInterface.CalcTheRoute` (`self.DroneBounds`) (`self.K2_GetActorLocation`) (`self.K2_GetActorLocation` (`GameplayStatics.GetPlayerCharacter` 0)) self))

(event `self.Sphere.OnComponentBeginOverlap`
  (params (OverlappedComponent :type "PrimitiveComponent Object Reference") (OtherActor :type "Actor Object Reference") (OtherComp :type "PrimitiveComponent Object Reference") (OtherBodyIndex :type Integer) (bFromSweep :type Boolean) (SweepResult :type "HitResult Structure (by ref)"))
  (if (`self.ActorHasTag` OtherActor "Player")
    (`Timeline|Timeline` :!via `PlayFromStart`
      (:`Finished`
        (`GameplayStatics.SpawnSoundAtLocation` "/Game/Fab/Free_Sounds_Pack/cue/Explosion_Medium_2-1_Cue.Explosion_Medium_2-1_Cue" (`self.K2_GetActorLocation`) (struct) 1.0 1.0 0.0 null null)
        (message `/Game/DamageSystem/BPI_Damagable.TakeDamage` OtherActor (make `/Game/DamageSystem/Struct/S_DamageInfo` 15.0 "NewEnumerator3" "NewEnumerator4" false false true) self (0.0 0.0 0.0) 0.0)
        (`self.Die`)))))

(event `self.Sphere.OnComponentEndOverlap`
  (params (OverlappedComponent :type "PrimitiveComponent Object Reference") (OtherActor :type "Actor Object Reference") (OtherComp :type "PrimitiveComponent Object Reference") (OtherBodyIndex :type Integer))
  (if (`self.ActorHasTag` OtherActor "Player")
    _))

(fn `UserConstructionScript`
  (`parent.UserConstructionScript`))