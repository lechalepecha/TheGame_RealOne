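; Enemy manager actor that tracks the level's enemy count and handles level completion.
; On BeginPlay it counts all BP_Enemy_Base actors; Tick watches for the count reaching zero, then once shows the player character's completion menu, switches to UI-only input and pauses the game.
; CanSearch throttles searches using a point-of-interest distance check and a cooldown since the last approved search.
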(event `self.ReceiveBeginPlay`
  (bind _outactors (`GameplayStatics.GetAllActorsOfClass` "/Game/Enemies/BP_Enemy_Base.BP_Enemy_Base_C"))
  (for _ _outactors
    (`/Engine/EditorBlueprintResources/StandardMacros.IncrementInt` (`self.EnemyCount`))))

(event `self.ReceiveTick`
  (params (DeltaSeconds :type "Float (single-precision)"))
  (if (not (> (`self.EnemyCount`) 0))
    (`/Engine/EditorBlueprintResources/StandardMacros.DoOnce` false
      (:`Completed`
        (bind _asbp_fpcharacter (cast `/Game/FirstPerson/Blueprints/BP_FPCharacter` (`GameplayStatics.GetPlayerCharacter` 0)))
        (bind _menucompleted (`/Game/FirstPerson/Blueprints/BP_FPCharacter.MenuCompleted` _asbp_fpcharacter))
        (`UserWidget.AddToViewport` _menucompleted 5)
        (bind _returnvalue (`Pawn.GetLocalViewingPlayerController` _asbp_fpcharacter))
        (set `PlayerController.bShowMouseCursor` true _returnvalue)
        (`WidgetBlueprintLibrary.SetInputMode_UIOnlyEx` _returnvalue _menucompleted)
        (`GameplayStatics.SetGamePaused` true)))))

(fn `CanSearch`
  (params (PointOfInterest :type "Vector Structure"))
  (returns (CanSearch :type Boolean))
  (if (> (`KismetMathLibrary.Vector_Distance` PointOfInterest (`self.PointOfInterest`)) 200.0)
    _
    (elif (> (- (`GameplayStatics.GetTimeSeconds`) (`self.SearchTime`)) 10.0)
      _
      (else
        (return false))))
  (set `self.PointOfInterest` PointOfInterest)
  (set `self.SearchTime` (`GameplayStatics.GetTimeSeconds`))
  (return true))

(fn `UserConstructionScript`)