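; Drone flight volume that builds a 3D navigation grid inside its box bounds.
; BeginPlay samples grid points, debug-draws them, and line-traces between neighbours from Variations offsets, storing linear indices and visibility.
; FindWay greedily steps to open neighbours using straight-line step cost plus heuristic, without an open list, then prints the path.
; It ignores its inputs, running first to last point, and its calls here are disconnected.
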(event `self.ReceiveBeginPlay`
  (bind _dotlocations (`self.DotLocations`))
  (bind _yarray (`self.YArray`))
  (bind _zarray (`self.ZArray`))
  (bind _returnvalue (`KismetArrayLibrary.Array_Length` _zarray))
  (bind _returnvalue_2 (`KismetArrayLibrary.Array_Length` _yarray))
  (bind _returnvalue_3 (+ (`self.ZIndex`) (* (`self.XIndex`) (* _returnvalue_2 _returnvalue)) (* (`self.YIndex`) _returnvalue)))
  (bind _output_location (break `/Game/Enemies/LocationInfo` (`|GetArrayItem` _dotlocations _returnvalue_3)))
  (bind _output_location_2 (break `/Game/Enemies/LocationInfo` (`|GetArrayItem` (`self.DotLocations`) _returnvalue_3)))
  (while (< (`self.XMin`) (`self.XMax`))
    (`KismetArrayLibrary.Array_Add` (`self.XArray`) (`self.XMin`))
    (set `self.XMin` (+ (`self.XMin`) (`self.Interaval`))))
  (while (< (`self.YMin`) (`self.YMax`))
    (`KismetArrayLibrary.Array_Add` (`self.YArray`) (`self.YMin`))
    (set `self.YMin` (+ (`self.YMin`) (`self.Interaval`))))
  (while (< (`self.ZMin`) (`self.ZMax`))
    (`KismetArrayLibrary.Array_Add` (`self.ZArray`) (`self.ZMin`))
    (set `self.ZMin` (+ (`self.ZMin`) (`self.Interaval`))))
  (for _index (range (+ (`KismetArrayLibrary.Array_LastIndex` (`self.XArray`)) 1))
    (for _index_2 (range (+ (`KismetArrayLibrary.Array_LastIndex` (`self.YArray`)) 1))
      (for _index_3 (range (+ (`KismetArrayLibrary.Array_LastIndex` (`self.ZArray`)) 1))
        (bind _output (`|GetArrayItem` (`self.XArray`) _index))
        (bind _output_2 (`|GetArrayItem` (`self.YArray`) _index_2))
        (bind _output_3 (`|GetArrayItem` (`self.ZArray`) _index_3))
        (`KismetArrayLibrary.Array_Add` (`self.DotLocations`) (make `/Game/Enemies/LocationInfo` (`KismetMathLibrary.MakeVector` _output _output_2 _output_3)))
        (`KismetSystemLibrary.SphereTraceSingle` :`Start` (`KismetMathLibrary.MakeVector` _output _output_2 _output_3) :`End` (`KismetMathLibrary.MakeVector` _output _output_2 _output_3) :`Radius` 10.0 :`TraceChannel` "TraceTypeQuery1" :`DrawDebugType` "ForDuration" :`DrawTime` 10000.0))))
  (for _index_4 (range (+ (`KismetArrayLibrary.Array_LastIndex` (`self.XArray`)) 1))
    (set `self.XIndex` _index_4)
    (for _index_5 (range (+ (`KismetArrayLibrary.Array_LastIndex` (`self.YArray`)) 1))
      (set `self.YIndex` _index_5)
      (for _index_6 (range (+ (`KismetArrayLibrary.Array_LastIndex` (`self.ZArray`)) 1))
        (set `self.ZIndex` _index_6)
        (for _index_7 (range (+ (`KismetArrayLibrary.Array_LastIndex` (`self.Variations`)) 1))
          (bind (_output_x _output_y _output_z) (`KismetMathLibrary.BreakVector` (`|GetArrayItem` (`self.Variations`) _index_7)))
          (bind _returnvalue_4 (+ (`KismetMathLibrary.Conv_Int64ToInt` (`KismetMathLibrary.Conv_DoubleToInt64` _output_x)) (`self.XIndex`)))
          (bind _returnvalue_5 (+ (`KismetMathLibrary.Conv_Int64ToInt` (`KismetMathLibrary.Conv_DoubleToInt64` _output_y)) (`self.YIndex`)))
          (bind _returnvalue_6 (+ (`KismetMathLibrary.Conv_Int64ToInt` (`KismetMathLibrary.Conv_DoubleToInt64` _output_z)) (`self.ZIndex`)))
          (if (and (>= _returnvalue_4 0) (>= _returnvalue_5 0) (>= _returnvalue_6 0) (<= _returnvalue_4 (`KismetArrayLibrary.Array_LastIndex` (`self.XArray`))) (<= _returnvalue_5 (`KismetArrayLibrary.Array_LastIndex` _yarray)) (<= _returnvalue_6 (`KismetArrayLibrary.Array_LastIndex` _zarray)))
            (bind _output_get (set `self.LinearIndex` (+ (* _returnvalue_4 (* _returnvalue_2 _returnvalue)) (* _returnvalue_5 _returnvalue) _returnvalue_6)))
            (bind _output_location_3 (break `/Game/Enemies/LocationInfo` (`|GetArrayItem` (`self.DotLocations`) _output_get)))
            (bind (_outhit _returnvalue_7) (`KismetSystemLibrary.LineTraceSingle` :`Start` _output_location_2 :`End` _output_location_3 :`TraceChannel` "TraceTypeQuery1" :`DrawTime` 50.0))
            (`KismetArrayLibrary.Array_Add` (`self.AccessabilityTemp`) (not _returnvalue_7))
            (`KismetArrayLibrary.Array_Add` (`self.NeighboursIndexTemp`) _output_get)))
        (`KismetArrayLibrary.Array_Set` _dotlocations _returnvalue_3 (make `/Game/Enemies/LocationInfo` _output_location (`self.AccessabilityTemp`) (`self.NeighboursIndexTemp`)))))))

(event `self.ReceiveTick`
  (params (DeltaSeconds :type "Float (single-precision)")))

(event `FindWay`
  (params (CurrentLocation :type "Vector Structure") (TargetLocation :type "Vector Structure"))
  (bind _currentlocation_location (break `/Game/Enemies/LocationInfo` (`self.CurrentLocation`)))
  (bind _dotlocations (`self.DotLocations`))
  (bind (_currentlocation_location_2 _currentlocation_neighbourlocations _currentlocation_neighbourlinearindex) (break `/Game/Enemies/LocationInfo` (`self.CurrentLocation`)))
  (bind _currentlocation_location_3 (break `/Game/Enemies/LocationInfo` (`self.CurrentLocation`)))
  (bind _endlocation (`self.EndLocation`))
  (bind (_currentlocation_location_4 _currentlocation_neighbourlocations_2 _currentlocation_neighbourlinearindex_2) (break `/Game/Enemies/LocationInfo` (`self.CurrentLocation`)))
  (bind _bestneighbour (`self.BestNeighbour`))
  (bind _dotlocations_2 (`self.DotLocations`))
  (bind _selectedlocations (`self.SelectedLocations`))
  (bind _output_location (break `/Game/Enemies/LocationInfo` (`|GetArrayItem` _dotlocations)))
  (bind _output_location_2 (break `/Game/Enemies/LocationInfo` (`|GetArrayItem` _dotlocations_2 (`KismetArrayLibrary.Array_LastIndex` _dotlocations_2))))
  (set `self.StartLocation` _output_location)
  (set `self.CurrentLocation` (`|GetArrayItem` _dotlocations))
  (bind _output_get (set `self.EndLocation` _output_location_2))
  (`KismetArrayLibrary.Array_Add` (`self.SelectedLocations`))
  (while (!= _output_get _currentlocation_location :`ErrorTolerance` 500.0)
    (bind _heuristics (`self.FindHeurisitcs` _currentlocation_location_3 _endlocation))
    (bind _stepcost (`self.FindStepCost` _currentlocation_location_3 _endlocation))
    (set `self.FinalPriority` (+ _stepcost _heuristics))
    (for _index (range (+ (`KismetArrayLibrary.Array_LastIndex` _currentlocation_neighbourlinearindex) 1))
      (if (`|GetArrayItem` _currentlocation_neighbourlocations_2 _index)
        (bind _output (`|GetArrayItem` _currentlocation_neighbourlinearindex_2 _index))
        (bind _output_location_3 (break `/Game/Enemies/LocationInfo` (`|GetArrayItem` (`self.DotLocations`) _output)))
        (bind _heuristics_2 (`self.FindHeurisitcs` _output_location_3 (`self.EndLocation`)))
        (bind _stepcost_2 (`self.FindStepCost` _currentlocation_location_4 _output_location_3))
        (bind _returnvalue (+ _heuristics_2 _stepcost_2))
        (if (< _returnvalue (`self.FinalPriority`))
          (set `self.FinalPriority` _returnvalue)
          (set `self.BestNeighbour` _output))))
    (`KismetArrayLibrary.Array_Add` (`self.SelectedLocations`) _bestneighbour)
    (set `self.CurrentLocation` (`|GetArrayItem` (`self.DotLocations`) _bestneighbour)))
  (`KismetArrayLibrary.Array_Add` _selectedlocations (`KismetArrayLibrary.Array_LastIndex` (`self.DotLocations`)))
  (for _index_2 (range (+ (`KismetArrayLibrary.Array_LastIndex` _selectedlocations) 1))
    (`KismetSystemLibrary.PrintString` (`KismetStringLibrary.Conv_IntToString` (`|GetArrayItem` (`self.SelectedLocations`) _index_2)) true true (struct :`G` 0.66 :`B` 1.0 :`A` 1.0) 100.0)))

(fn `FindHeurisitcs`
  (params (CurrentLocation :type "Vector Structure") (EndLocation :type "Vector Structure"))
  (returns (Heuristics :type "Float (double-precision)"))
  (return (`KismetMathLibrary.Sqrt` (+ (`KismetMathLibrary.Square` (- CurrentLocation_X EndLocation_X)) (`KismetMathLibrary.Square` (- CurrentLocation_Y EndLocation_Y)) (`KismetMathLibrary.Square` (- CurrentLocation_Z EndLocation_Z))))))

(fn `FindStepCost`
  (params (CurrentLocation :type "Vector Structure") (NextLocation :type "Vector Structure"))
  (returns (StepCost :type "Float (double-precision)"))
  (return (`KismetMathLibrary.Sqrt` (+ (`KismetMathLibrary.Square` (- NextLocation_X CurrentLocation_X)) (`KismetMathLibrary.Square` (- NextLocation_Y CurrentLocation_Y)) (`KismetMathLibrary.Square` (- NextLocation_Z CurrentLocation_Z))))))

(fn `UserConstructionScript`
  (bind (_origin _boxextent) (`KismetSystemLibrary.GetComponentBounds` (`self.Box`)))
  (`BoxComponent.SetBoxExtent` (`self.Box`) (`SceneComponent.RelativeScale3D` (`self.DefaultSceneRoot`)) true)
  (set `self.XMin` (- (.x _origin) (.x _boxextent)))
  (set `self.XMax` (+ (.x _origin) (.x _boxextent)))
  (set `self.YMin` (- (.y _origin) (.y _boxextent)))
  (set `self.YMax` (+ (.y _origin) (.y _boxextent)))
  (set `self.ZMin` (- (.z _origin) (.z _boxextent)))
  (set `self.ZMax` (+ (.z _origin) (.z _boxextent))))