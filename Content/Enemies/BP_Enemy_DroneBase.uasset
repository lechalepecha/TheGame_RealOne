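; Base flying drone enemy that follows a waypoint route within DroneBounds, with child classes expected to implement the route calculation called every second.
; Tick steers CharacterMovement velocity toward a speed-scaled look-ahead point, blending ray-fan obstacle avoidance, slerp-limited turning and slowdown near waypoints or sharp turns.
; BPC damage component handles health and death, which stops AI logic and destroys the actor.
; Most other enemy functions are stubs, and debug drawing is active.
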(event `self.ReceiveActorBeginOverlap`
  (params (OtherActor :type "Actor Object Reference")))

(event `self.ReceiveBeginPlay`
  (bind _bpc_damagesystem (`self.BPC_DamageSystem`))
  (bind _returnvalue (`NavBoundsManager.FindBestNavBounds` (subsystem `NavBoundsManager`) (`self.K2_GetActorLocation`)))
  (bind _output_get (set `self.DroneBounds` _returnvalue))
  (`KismetSystemLibrary.Delay` 0.2)
  (bind _asdrone_bounds (cast `/Game/Enemies/DroneBounds` _output_get))
  (set `self.DroneBounds` _asdrone_bounds)
  (`KismetSystemLibrary.K2_SetTimerDelegate` (delegate `CallCalcTheRoute`) 1.0 true)
  (bind _asaic_enemy_drone (cast `/Game/Enemies/AI/AIC_Enemy_Drone` (`AIBlueprintHelperLibrary.GetAIController` self))
    (:`then`
      (set `self.AIC Enemy Drone` _asaic_enemy_drone)
      (add `/Game/DamageSystem/AC_DamageSystem.OnDeath` _bpc_damagesystem (`|CreateDelegate` :!event `Die`))
      (add `/Game/DamageSystem/AC_DamageSystem.OnDamageResponce` _bpc_damagesystem (`|CreateDelegate` :!event `RespondDamage`)))
    (:`CastFailed`
      (`KismetSystemLibrary.PrintString` "Cast to AI controller failed"))))

(event `CallCalcTheRoute`
  ;[1 1 1] Set needed implementation in child
)

(event `FlyingNavigationInterface.GetTheRouteInLocations`
  (params (RouteInLocations :type "Array of Vector Structure (by ref)"))
  (set `self.Route in Locations` RouteInLocations)
  (bind _result (`/Engine/EditorBlueprintResources/StandardMacros.DecrementInt` (`KismetArrayLibrary.Array_LastIndex` RouteInLocations))
    (:`  `
      (for _index (range (+ _result 1))
        (`KismetSystemLibrary.DrawDebugLine` (`|GetArrayItem` RouteInLocations _index) (`|GetArrayItem` RouteInLocations (+ _index 1)) (struct :`R` 1.0 :`B` 0.168417 :`A` 1.0) 1.0 10.0)))))

(event `self.ReceiveTick`
  (params (DeltaSeconds :type "Float (single-precision)"))
  (`self.MoveAlongTheRoute` DeltaSeconds))

(event `Die`
  (bind _mesh (`self.Mesh`))
  (`BrainComponent.StopLogic` (`AIController.BrainComponent` (`self.AIC Enemy Drone`)) "")
  (`PrimitiveComponent.SetCollisionResponseToChannel` (`self.Mesh`) "ECC_Pawn" "ECR_Overlap")
  (`MovementComponent.StopMovementImmediately` (`self.CharacterMovement`))
  (`PrimitiveComponent.SetCollisionEnabled` _mesh "QueryAndPhysics")
  (`PrimitiveComponent.SetSimulatePhysics` _mesh true)
  (`PrimitiveComponent.SetCollisionEnabled` (`self.CapsuleComponent`) "NoCollision")
  (`self.K2_DestroyActor`))

(event `RespondDamage`
  (params (DamageResponce :type "/Game/DamageSystem/Enum/E_DamageResponce Enum" :default "NewEnumerator0") (DamageCuaser :type "Actor Object Reference") (KnockbackEpicenter :type "Vector Structure") (HitBoneName :type Name) (DamageDirection :type "/Game/DamageSystem/Enum/E_DamageDirection Enum" :default "NewEnumerator0")))

(fn `CalculateLookAheadPoint`
  (returns (Waypoint :type "Vector Structure"))
  (locals (CurrentPos :type "Vector Structure") (DynamicLookAhead :type "Float (double-precision)") (Idx :type Integer) (RemainingDist :type "Float (double-precision)") (LastWaypoint :type "Vector Structure") (NextPoint :type "Vector Structure") (SegmentLength :type "Float (double-precision)"))
  (bind _remainingdist (`local.RemainingDist`))
  (bind _route_in_locations (`self.Route in Locations`))
  (set `local.CurrentPos` (`self.K2_GetActorLocation`))
  (set `local.DynamicLookAhead` (+ (`self.LookAheadDistance`) (* (`KismetMathLibrary.VSize` (`self.CurrentVelocity`)) 0.5)))
  (set `local.Idx` (`self.WaypointIndex`))
  (set `local.RemainingDist` (`local.DynamicLookAhead`))
  (set `local.LastWaypoint` (`|GetArrayItem` (`self.Route in Locations`) (`local.Idx`)))
  (while (and (< (`local.Idx`) (`KismetArrayLibrary.Array_Length` (`self.Route in Locations`))) (> (`local.RemainingDist`) 0.0))
    (bind _output_get (set `local.NextPoint` (`|GetArrayItem` (`self.Route in Locations`) (+ (`local.Idx`) 1))))
    (bind _output_get_2 (set `local.SegmentLength` (`KismetMathLibrary.VSize` (- _output_get (`local.LastWaypoint`)))))
    (if (<= _remainingdist _output_get_2)
      (return (`KismetMathLibrary.VLerp` (`local.LastWaypoint`) (`local.NextPoint`) (/ _remainingdist _output_get_2)))
      (else
        (set `local.RemainingDist` (- (`local.RemainingDist`) (`local.SegmentLength`)))
        (set `local.LastWaypoint` (`local.NextPoint`))
        (`/Engine/EditorBlueprintResources/StandardMacros.IncrementInt` (`local.Idx`)))))
  (return (`|GetArrayItem` _route_in_locations (`KismetArrayLibrary.Array_LastIndex` _route_in_locations))))

(fn `CalculateTargetSpeed`
  (params (DisctanceToWaypoint :type "Float (double-precision)") (TurnAngle :type "Float (double-precision)"))
  (returns (Speed :type "Float (double-precision)"))
  (locals (TargetSpeed :type "Float (double-precision)") (TurnFactor :type "Float (double-precision)") (TurnSpeedReduction :type "Float (double-precision)"))
  (set `local.TargetSpeed` (`self.MaxSpeed`))
  (if (< DisctanceToWaypoint (`self.SlowdownRadius`))
    (set `local.TargetSpeed` (`KismetMathLibrary.Lerp` (`self.MinSpeed`) (`self.MaxSpeed`) (`KismetMathLibrary.FClamp` (/ DisctanceToWaypoint (`self.SlowdownRadius`))))))
  (if (> TurnAngle 15.0)
    (bind _output_get (set `local.TurnFactor` (`KismetMathLibrary.FClamp` (/ TurnAngle 90.0))))
    (bind _output_get_2 (set `local.TurnSpeedReduction` (* _output_get (`self.TurnSlowdownFactor`))))
    (bind _output_get_3 (set `local.TargetSpeed` (* (`local.TargetSpeed`) (- 1.0 _output_get_2)))))
  (return (`KismetMathLibrary.FMax` _output_get_3 (`self.MinSpeed`))))

(fn `GetClosestWaypoint`
  (returns (WaypointIndex :type Integer))
  (locals (CurrentWaypointDistance :type "Float (double-precision)") (WaypointIDx :type Integer))
  (bind _returnvalue (`KismetMathLibrary.Vector_Distance` (`|GetArrayItem` (`self.Route in Locations`) (`self.WaypointIndex`)) (`self.K2_GetActorLocation`)))
  (if (> _returnvalue (`self.MaxWaypointDistance`))
    (set `local.CurrentWaypointDistance` _returnvalue)
    (for _index (range (+ (`KismetArrayLibrary.Array_LastIndex` (`self.Route in Locations`)) 1))
      (bind _returnvalue_2 (`KismetMathLibrary.Vector_Distance` (`|GetArrayItem` (`self.Route in Locations`) _index) (`self.K2_GetActorLocation`)))
      (if (> (`local.CurrentWaypointDistance`) _returnvalue_2)
        (set `local.CurrentWaypointDistance` _returnvalue_2)
        (set `local.WaypointIDx` _index)))
    (return (`local.WaypointIDx`))))

(fn `GetCurrentHealth`
  (returns (Health :type "Float (double-precision)"))
  (return (`/Game/DamageSystem/AC_DamageSystem.Health` (`self.BPC_DamageSystem`))))

(fn `GetFocusPoint`
  (returns (FocusActor :type "Actor Object Reference"))
  (return null))

(fn `GetIdealRange`
  (returns (AttackRadius :type "Float (double-precision)") (DefendRadius :type "Float (double-precision)"))
  (return 500.0 50.0))

(fn `GetMaxHealth`
  (returns (MaxHealth :type "Float (double-precision)"))
  (return (`/Game/DamageSystem/AC_DamageSystem.MaxHealth` (`self.BPC_DamageSystem`))))

(fn `GetPatrolRoute`
  (returns (PatrolRoute :type "/Game/Enemies/AI/Routes/BP_PatrolRoute Object Reference"))
  (return null))

(fn `Heal`
  (params (Ammount :type "Float (double-precision)"))
  (returns (NewHealth :type "Float (double-precision)"))
  (return 0.0))

(fn `IsDead`
  (returns (IsDead :type Boolean))
  (return (`/Game/DamageSystem/AC_DamageSystem.IsDead` (`self.BPC_DamageSystem`))))

(fn `Limit Turn Rate`
  (params (CurrentDir :type "Vector Structure") (DesiredDir :type "Vector Structure") (DeltaTime :type "Float (double-precision)"))
  (returns (TurnRate :type "Vector Structure"))
  (locals (DotProd :type "Float (double-precision)") (AngleDifference :type "Float (double-precision)") (MaxAngleThisFrame :type "Float (double-precision)") (CurrentQuat :type "Quat Structure") (DesiredQuat :type "Quat Structure") (Result :type "Quat Structure"))
  (bind _returnvalue (`KismetMathLibrary.Conv_VectorToQuaternion` (`local.DesiredDir`)))
  (bind _returnvalue_2 (`KismetMathLibrary.Conv_VectorToQuaternion` (`local.CurrentDir`)))
  (bind _output_get (set `local.DotProd` (`KismetMathLibrary.FClamp` (`KismetMathLibrary.Dot_VectorVector` CurrentDir DesiredDir) -1.0)))
  (set `local.AngleDifference` (`KismetMathLibrary.RadiansToDegrees` (`KismetMathLibrary.Acos` _output_get)))
  (bind _output_get_2 (set `local.MaxAngleThisFrame` (* (`self.MaxTurnRate`) DeltaTime)))
  (if (<= (`local.AngleDifference`) _output_get_2)
    (return (`local.DesiredDir`))
    (else
      (set `local.CurrentQuat` _returnvalue_2)
      (set `local.DesiredQuat` _returnvalue)
      (bind _output_get_3 (set `local.Result` (`KismetMathLibrary.Quat_Slerp` _returnvalue_2 _returnvalue (/ (`local.MaxAngleThisFrame`) (`local.AngleDifference`)))))
      (return (`KismetMathLibrary.Quat_VectorForward` _output_get_3)))))

(fn `MoveAlongTheRoute`
  (params (DeltaTime :type "Float (double-precision)"))
  (locals (CurrentPos :type "Vector Structure") (LookAheadPoint :type "Vector Structure") (DesiredDirection :type "Vector Structure") (CurrentDirection :type "Vector Structure") (NewDirection :type "Vector Structure") (Delta :type "Float (double-precision)") (CurrenWaypoint :type "Vector Structure") (DistToWaypoint :type "Float (double-precision)") (TurnAngle :type "Float (double-precision)") (TagetSpeed :type "Float (double-precision)") (NewLocalVar :type "Float (double-precision)") (CurrentSpeed :type "Float (double-precision)") (NewSpeed :type "Float (double-precision)") (TargetRotation :type "Rotator Structure") (NewRotation :type "Rotator Structure"))
  (bind _currentdirection (`local.CurrentDirection`))
  (bind _desireddirection (`local.DesiredDirection`))
  (set `local.Delta` DeltaTime)
  (if (not (< (`KismetArrayLibrary.Array_Length` (`self.Route in Locations`)) 2))
    (bind _output_get (set `local.CurrentPos` (`self.K2_GetActorLocation`)))
    (bind _waypoint (`self.CalculateLookAheadPoint`))
    (bind _output_get_2 (set `local.LookAheadPoint` _waypoint))
    (bind _avoidancevector (`self.Obstacle Avoidance`))
    (bind _output_get_3 (set `local.DesiredDirection` (`KismetMathLibrary.Normal` (- _output_get_2 _output_get))))
    (bind _output_get_4 (set `self.ObstacleAvoidance` _avoidancevector))
    (set `local.DesiredDirection` (`KismetMathLibrary.Normal` (+ _output_get_4 _output_get_3)))
    (set `local.CurrentDirection` (`KismetMathLibrary.Normal` (`self.CurrentVelocity`)))
    (if (< (`KismetMathLibrary.VSizeSquared` (`self.CurrentVelocity`)) 1.0)
      (bind _output_get_5 (set `local.CurrentDirection` (`local.DesiredDirection`)))
      (set `self.CurrentVelocity` (* _output_get_5 (`self.MinSpeed`))))
    (bind _turnrate (`self.Limit Turn Rate` _currentdirection _desireddirection (`local.Delta`)))
    (set `local.NewDirection` _turnrate)
    (bind _output_get_6 (set `local.CurrenWaypoint` (`|GetArrayItem` (`self.Route in Locations`) (`self.WaypointIndex`))))
    (bind _output_get_7 (set `local.DistToWaypoint` (`KismetMathLibrary.VSize` (- _output_get_6 (`local.CurrentPos`)))))
    (bind _output_get_8 (set `local.TurnAngle` (`KismetMathLibrary.RadiansToDegrees` (`KismetMathLibrary.Acos` (`KismetMathLibrary.FClamp` (`KismetMathLibrary.Dot_VectorVector` _currentdirection _desireddirection) -1.0)))))
    (bind _speed (`self.CalculateTargetSpeed` _output_get_7 _output_get_8))
    (bind _output_get_9 (set `local.TagetSpeed` _speed))
    (bind _output_get_10 (set `local.CurrentSpeed` (`KismetMathLibrary.VSize` (`MovementComponent.Velocity` (`self.CharacterMovement`)))))
    (bind _output_get_11 (set `local.NewSpeed` (`KismetMathLibrary.FInterpTo` _output_get_10 _output_get_9 (`local.Delta`) 75.0)))
    (bind _output_get_12 (set `self.CurrentVelocity` (* (`local.NewDirection`) _output_get_11)))
    (set `MovementComponent.Velocity` _output_get_12 (`self.CharacterMovement`))
    (if (> (`KismetMathLibrary.VSizeSquared` _output_get_12) 100.0)
      (bind _output_get_13 (set `local.TargetRotation` (`KismetMathLibrary.Conv_VectorToRotator` _output_get_12)))
      (bind _output_get_14 (set `local.NewRotation` (`KismetMathLibrary.RInterpTo` (`self.K2_GetActorRotation`) _output_get_13 (`local.Delta`) 100.0)))
      (`self.K2_SetActorRotation` _output_get_14 true))
    (`self.UpdateWaypointIndex`)))

(fn `Obstacle Avoidance`
  (returns (AvoidanceVector :type "Vector Structure"))
  (locals (CurrentLoc :type "Vector Structure") (CurrentDir :type "Vector Structure") (Avoidance :type "Vector Structure") (AngleOffset :type "Float (double-precision)") (Rotation :type "Quat Structure") (RayDirection :type "Vector Structure") (AvoidDir :type "Vector Structure"))
  (bind _returnvalue (`self.K2_GetActorLocation`))
  (bind _avoidance (`local.Avoidance`))
  (bind _horizontalavoidanceangle (`self.HorizontalAvoidanceAngle`))
  (bind (_raydirection_x _raydirection_y) (`KismetMathLibrary.BreakVector` (`local.RayDirection`)))
  (bind _verticalavoidanceangle (`self.VerticalAvoidanceAngle`))
  (bind _currentloc (`local.CurrentLoc`))
  (set `local.CurrentLoc` (`self.K2_GetActorLocation`))
  (set `local.CurrentDir` (`KismetMathLibrary.Normal` (`self.CurrentVelocity`)))
  (set `local.Avoidance` (0.0 0.0 0.0))
  (for _index (range (+ (`self.AvoidanceHorizontalRays`) 1))
    (bind _output_get (set `local.AngleOffset` (`KismetMathLibrary.Lerp` (* _horizontalavoidanceangle -1.0) _horizontalavoidanceangle (/ (`KismetMathLibrary.Conv_IntToDouble` _index) (`KismetMathLibrary.Conv_IntToDouble` (`self.AvoidanceHorizontalRays`))))))
    (set `local.RayDirection` (`KismetMathLibrary.RotateAngleAxis` (`local.CurrentDir`) _output_get (`self.GetActorUpVector`)))
    (for _index_2 (range (+ (`self.AvoidanceVerticalRays`) 1))
      (bind _output_get_2 (set `local.AngleOffset` (`KismetMathLibrary.Lerp` (* _verticalavoidanceangle -1.0) _verticalavoidanceangle (/ (`KismetMathLibrary.Conv_IntToDouble` _index_2) (`KismetMathLibrary.Conv_IntToDouble` (`self.AvoidanceVerticalRays`))))))
      (bind (_returnvalue_x _returnvalue_y _returnvalue_z) (`KismetMathLibrary.BreakVector` (`KismetMathLibrary.RotateAngleAxis` (`local.CurrentDir`) _output_get_2 (`KismetMathLibrary.Cross_VectorVector` (`self.GetActorUpVector`) (`self.GetActorForwardVector`)))))
      (bind _output_get_3 (set `local.RayDirection` (+ (`KismetMathLibrary.MakeVector` 0.0 0.0 _returnvalue_z) (`KismetMathLibrary.MakeVector` _raydirection_x _raydirection_y))))
      (bind (_outhit _returnvalue_2) (`KismetSystemLibrary.LineTraceSingle` :`Start` _currentloc :`End` (+ _currentloc (* _output_get_3 (`self.ObstacleCheckDistance`))) :`TraceChannel` "TraceTypeQuery1" :`bTraceComplex` true :`DrawDebugType` "ForDuration" :`DrawTime` 0.05))
      (if _returnvalue_2
        (bind _output_get_4 (set `local.AvoidDir` (* (`local.RayDirection`) -1.0)))
        (bind _returnvalue_3 (/ (`.Distance` (`GameplayStatics.BreakHitResult` _outhit)) (`self.ObstacleCheckDistance`)))
        (set `local.Avoidance` (+ (`local.Avoidance`) (* _output_get_4 (- 1.0 _returnvalue_3) (`self.AvoidanceForce`))))
        (else
          (bind _output_get_5 (set `local.AvoidDir` (* (`local.RayDirection`) -1.0)))
          (set `local.Avoidance` (- (`local.Avoidance`) (* _output_get_5 (- 1.0 _returnvalue_3) (`self.AvoidanceForce`))))))))
  (`KismetSystemLibrary.DrawDebugLine` _returnvalue (+ _returnvalue (* _avoidance 1.0)) (struct :`G` 0.153307 :`B` 1.0 :`A` 1.0) 0.1 5.0)
  (return _avoidance))

(fn `ReserveAttackToken`
  (params (Amount :type Integer))
  (returns (Success :type Boolean))
  (return false))

(fn `StartAttack`
  (params (AttackTarget :type "Actor Object Reference") (TokensNeeded :type Integer))
  (returns (Success :type Boolean))
  (return false))

(fn `TakeDamage`
  (params (DamageInfo :type "/Game/DamageSystem/Struct/S_DamageInfo Structure") (DamageCauser :type "Actor Object Reference") (`Knockback Epicenter` :type "Vector Structure") (DamageDuration :type "Float (double-precision)"))
  (returns (WasDamaged :type Boolean) (WasDamagedToDeath :type Boolean) (FinalDamage :type "Float (double-precision)") (IsCriticalHit :type Boolean))
  (if (not (`|EnumEquality` (`.DamageResponce_16_923A35E345F2219B8E18CBA5D7476FD8` (break `/Game/DamageSystem/Struct/S_DamageInfo` DamageInfo)) "NewEnumerator8"))
    (bind (_wasdamaged _wasdamagedtodeath _finaldamage _iscriticalhit) (`/Game/DamageSystem/AC_DamageSystem.TakeDamage` (`self.BPC_DamageSystem`) DamageInfo DamageCauser `Knockback Epicenter`))
    (if _wasdamaged
      (return _wasdamaged _wasdamagedtodeath _finaldamage _iscriticalhit))))

(fn `UpdateMovementSpeed`
  (params (SpeedType :type "/Game/Enemies/AI/Enums/E_MovementSpeed Enum" :default "NewEnumerator0"))
  (returns (`Speed Value` :type "Float (double-precision)"))
  (return 0.0))

(fn `UpdateState`
  (params (NewState :type "/Game/Enemies/AI/Enums/E_EnemyStates Enum" :default "NewEnumerator0"))
  (returns (State :type "/Game/Enemies/AI/Enums/E_EnemyStates Enum"))
  (return "NewEnumerator0"))

(fn `UpdateWaypointIndex`
  (locals (CurrentPos :type "Vector Structure") (CurrentWaypoint :type "Vector Structure") (Distance :type "Float (double-precision)") (NextId :type Integer) (NextWP :type "Vector Structure"))
  (bind _output_get (set `local.CurrentPos` (`self.K2_GetActorLocation`)))
  (bind _output_get_2 (set `local.CurrentWaypoint` (`|GetArrayItem` (`self.Route in Locations`) (`self.WaypointIndex`))))
  (set `local.Distance` (`KismetMathLibrary.VSize` (- _output_get_2 _output_get)))
  (bind _output_get_3 (set `local.NextId` (`KismetMathLibrary.Min` (+ (`self.WaypointIndex`) 1) (`KismetArrayLibrary.Array_LastIndex` (`self.Route in Locations`)))))
  (set `local.NextWP` (`|GetArrayItem` (`self.Route in Locations`) _output_get_3))
  (if (and (< (`local.Distance`) (`self.WaypoinReachedRadius`)) (> (`KismetMathLibrary.Abs` (`KismetMathLibrary.Dot_VectorVector` (`KismetMathLibrary.Normal` (- (`local.CurrentWaypoint`) (`local.NextWP`))) (- (`local.CurrentPos`) (`local.CurrentWaypoint`)))) 50.0))
    (bind _result (`/Engine/EditorBlueprintResources/StandardMacros.IncrementInt` (`self.WaypointIndex`))
      (:`  `
        (if (>= _result (`KismetArrayLibrary.Array_Length` (`self.Route in Locations`)))
          (set `self.WaypointIndex` 0))))))

(fn `UserConstructionScript`)