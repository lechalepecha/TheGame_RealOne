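; Ranged, weapon-wielding enemy Blueprint for the invisible drone, supplying combat ranges, movement speeds and attack-token handling.
; It equips a pooled weapon through ACWeaponPool, attaching it to the hand socket and linking its anim layers.
; RangedAttack handles busy and empty-magazine states, then fires by fire mode using timers and a randomized burst length.
; Weapon-wielder callbacks play montages, emit AI noise on firing and report a constant, effectively infinite ammo reserve.
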(event `self.ReceiveBeginPlay`
  (`parent.ReceiveBeginPlay`))

(event `self.AttachWeapon`
  (params (Weapon :type "TP_WeaponComponent Object Reference"))
  (bind _currentweapon (`self.CurrentWeapon`))
  (bind _currentweapon_2 (`self.CurrentWeapon`))
  (`TP_WeaponComponent.SetOwningWeaponWielder` Weapon self)
  (if (not (== (`self.CurrentWeapon`) Weapon))
    (`TP_WeaponComponent.SetIsEquippingFalse` Weapon)
    (set `TP_WeaponComponent.IsEquipping` true Weapon)
    (`SceneComponent.K2_AttachToComponent` Weapon (`self.Mesh`) "weapon_r" "SnapToTarget" "SnapToTarget" "SnapToTarget" true)
    (bind _output_get (set `self.CurrentWeapon` Weapon))
    (bind (_tptransform_location _tptransform_rotation) (`KismetMathLibrary.BreakTransform` (`TP_WeaponComponent.TPTransform` _output_get)))
    (`SceneComponent.K2_AddRelativeRotation` _output_get _tptransform_rotation false false)
    (`TP_WeaponComponent.Equip` _output_get)
    (`SkeletalMeshComponent.LinkAnimClassLayers` (`self.Mesh`) (`TP_WeaponComponent.TPWeaponAnimLinkLayer` _output_get))
    (`|PlayMontage` (`self.Mesh`) (`TP_WeaponComponent.TPEquipAnimation` (`self.CurrentWeapon`))
      (:`then`
        (set `self.IsWeaponEquiped` true)
        (set `TP_WeaponComponent.CanFire` true _currentweapon_2)
        (`TP_WeaponComponent.OnEquipDelegate` _currentweapon_2 self _currentweapon_2))
      (:`OnBlendOut`
        (`TP_WeaponComponent.EquipAnimationBlendOut` _currentweapon (`TP_WeaponComponent.TPEquipAnimation` _currentweapon) false)))))

(event `self.OnStow`
  (set `self.IsWeaponEquiped` false)
  (set `self.CurrentWeapon` null)
  (`self.OnWeaponUnequipped`))

(event `self.DetachWeapon`
  (bind _currentweapon (`self.CurrentWeapon`)
    (:`then`
      (set `TP_WeaponComponent.IsStowing` true _currentweapon)
      (bind _adstl (`TP_WeaponComponent.ADSTL` _currentweapon))
      (`TimelineComponent.SetNewTime` _adstl 0.0)
      (`TimelineComponent.Stop` _adstl)
      (`|PlayMontage` (`self.Mesh`) "/Game/Characters/Heroes/Mannequin/Animations/Actions/AM_MM_Generic_Unequip.AM_MM_Generic_Unequip"
        (:`OnCompleted`
          _)
        (:`OnInterrupted`
          _))
      (`TP_WeaponComponent.Stow` _currentweapon))
    (:`else`)))

(event `self.EquipWeapon`
  (`/Game/DamageSystem/Weapons/ObjectPool/AC_WeaponPool.SpawnFromPool` (`self.AC_WeaponPool`) 0)
  (`self.OnWeaponEquipped`))

(event `self.ForceStopAttacking`
  (bind _currentweapon (`self.CurrentWeapon`)
    (:`then`
      (`TP_WeaponComponent.ForceStopFire` _currentweapon))
    (:`else`
      (`self.On Attack End`))))

(event `self.OnStopFiring`
  (`self.AttackEnd` (stale `self.RangedAttack` AttackTarget)))

(event `self.UnequipWeapon`
  (`self.CurrentWeapon`
    (:`then`
      (`self.DetachWeapon`)
      (`SkeletalMeshComponent.LinkAnimClassLayers` (`self.Mesh`) "/Game/Characters/Heroes/Mannequin/Animations/Locomotion/Unarmed/ABP_UnarmedAnimLayers.ABP_UnarmedAnimLayers_C"))
    (:`else`)))

(event `self.RangedAttack`
  (params (AttackTarget :type "Actor Object Reference"))
  (bind _currentweapon (`self.CurrentWeapon`))
  (bind _currentweapon_2 (`self.CurrentWeapon`))
  (bind _currentweapon_3 (`self.CurrentWeapon`))
  (bind _currentweapon_4 (`self.CurrentWeapon`))
  (bind _currentweapon_5 (`self.CurrentWeapon`)
    (:`then`
      (set `TP_WeaponComponent.BurstFireRounds` (`KismetMathLibrary.RandomIntegerInRange` 2 5) _currentweapon_5)
      (set `TP_WeaponComponent.IsWielderHoldingShootButton` true (`self.CurrentWeapon`))
      (if (or (`TP_WeaponComponent.IsReloading` _currentweapon) (`TP_WeaponComponent.IsStowing` _currentweapon) (`TP_WeaponComponent.IsEquipping` _currentweapon) (> (`KismetSystemLibrary.K2_GetTimerRemainingTimeHandle` (`TP_WeaponComponent.FireRateDelayTimerHandle` _currentweapon)) 0.0))
        (`TP_WeaponComponent.StopFire` (`self.CurrentWeapon`))
        (`/Game/Enemies/AI/BPI_EnemyAI.ForceStopAttacking`)
        (elif (<= (`TP_WeaponComponent.CurrentMagazineCount` (`self.CurrentWeapon`)) 0)
          (set `TP_WeaponComponent.IsWielderHoldingShootButton` false _currentweapon_2)
          (`GameplayStatics.SpawnSoundAttached` (`TP_WeaponComponent.DryFireSound` _currentweapon_2) _currentweapon_2 "None" (0.0 0.0 0.0) (struct) "KeepRelativeOffset" false 1.0 1.0 0.0 null null)
          (bind _returnvalue (`WeaponWielderInterface.GetRemainingAmmo` self))
          (if (> _returnvalue 0)
            (`TP_WeaponComponent.Reload` _currentweapon_3)
            (`TP_WeaponComponent.StopFire` _currentweapon_3)
            (else
              (`TP_WeaponComponent.StopFire` _currentweapon_3)))
          (else
            (`KismetSystemLibrary.K2_ClearAndInvalidateTimerHandle` (`TP_WeaponComponent.FireRateDelayTimerHandle` (`self.CurrentWeapon`)))
            (`TP_WeaponComponent.RecoilStart` _currentweapon_4)
            (switch `EFireMode` (`TP_WeaponComponent.FireMode` _currentweapon_4)
              (:`Single`
                (`TP_WeaponComponent.SingleFire` (`self.CurrentWeapon`))
                (bind _returnvalue_2 (`KismetSystemLibrary.K2_SetTimerDelegate` :`Time` (`TP_WeaponComponent.FireDelay` (`self.CurrentWeapon`))))
                (set `TP_WeaponComponent.FireRateDelayTimerHandle` _returnvalue_2 (`self.CurrentWeapon`)))
              (:`Alternate`
                (bind _returnvalue_3 (`KismetSystemLibrary.K2_SetTimerDelegate` (delegate `StartAlternateFire`) (`TP_WeaponComponent.FireDelay` (`self.CurrentWeapon`)) true))
                (set `TP_WeaponComponent.FireRateDelayTimerHandle` _returnvalue_3 (`self.CurrentWeapon`)))
              (:`Burst`
                (bind _returnvalue_4 (`KismetSystemLibrary.K2_SetTimerDelegate` (delegate `StartBurstFire`) (`TP_WeaponComponent.FireDelay` (`self.CurrentWeapon`)) true))
                (set `TP_WeaponComponent.FireRateDelayTimerHandle` _returnvalue_4 (`self.CurrentWeapon`)))
              (:`Auto`
                (bind _returnvalue_5 (`KismetSystemLibrary.K2_SetTimerDelegate` (delegate `StartAutoFire`) (`TP_WeaponComponent.FireDelay` (`self.CurrentWeapon`)) true))
                (set `TP_WeaponComponent.FireRateDelayTimerHandle` _returnvalue_5 (`self.CurrentWeapon`))
                (`self.AttackEnd` AttackTarget)))))))
    (:`else`
      (`/Game/Enemies/AI/BPI_EnemyAI.ForceStopAttacking`))))

(event `self.OnWeaponStopReloadAnimation`
  (params (blendTime :type "Float (single-precision)"))
  (`AnimInstance.Montage_Stop` (`SkeletalMeshComponent.GetAnimInstance` (`self.Mesh`)) blendTime (`TP_WeaponComponent.TPReloadAnimation` (`self.CurrentWeapon`))))

(event `self.OnWeaponFired`
  (`|PlayMontage` (`self.Mesh`) (`TP_WeaponComponent.TPFireAnimation` (`self.CurrentWeapon`))
    (:`then`
      (`self.MakeNoise` 1.0 null (`SceneComponent.K2_GetComponentLocation` (`self.CurrentWeapon`))))))

(event `StartAlternateFire`
  (`TP_WeaponComponent.AlternateFire` (`self.CurrentWeapon`)))

(event `StartBurstFire`
  (`TP_WeaponComponent.BurstFire` (`self.CurrentWeapon`)))

(event `self.OnWeaponReload`
  (bind _currentweapon (`self.CurrentWeapon`))
  (set `TP_WeaponComponent.IsReloading` true _currentweapon)
  (`|PlayMontage` (`self.Mesh`) (`TP_WeaponComponent.TPReloadAnimation` _currentweapon)
    (:`OnCompleted`
      (set `TP_WeaponComponent.IsReloading` false _currentweapon))))

(event `self.SetWielderControlRotation`
  (params (newRotator :type "Rotator Structure"))
  (`Controller.SetControlRotation` (`self.GetController`) newRotator))

(event `StartAutoFire`
  (`TP_WeaponComponent.FullAutoFire` (`self.CurrentWeapon`)))

(event `self.OnReloadSuccess`
  (bind _currentweapon (`self.CurrentWeapon`))
  (`TP_WeaponComponent.OnReloaded` _currentweapon)
  (`TP_WeaponComponent.SetIsReloadingFalse` _currentweapon))

(event `self.ReturnAttackToken`
  (params (Amount :type Integer))
  (`/Game/DamageSystem/AC_DamageSystem.ReturnAttackToken` (`self.BPC_DamageSystem`) Amount))

(event `self.StoreAttackTokens`
  (params (AttackTarget :type "Actor Object Reference") (TokensAmount :type Integer))
  (bind (_value _returnvalue) (`BlueprintMapLibrary.Map_Find` (`self.ReservedAttackTokens`) AttackTarget))
  (`BlueprintMapLibrary.Map_Add` (`self.ReservedAttackTokens`) AttackTarget (`KismetMathLibrary.SelectInt` (+ TokensAmount _value) TokensAmount _returnvalue)))

(fn `GetCurrentWeapon`
  (returns (ReturnValue :type "TP_WeaponComponent Object Reference"))
  (return (`self.CurrentWeapon`)))

(fn `GetIdealRange`
  (returns (AttackRadius :type "Float (double-precision)") (DefendRadius :type "Float (double-precision)"))
  (return 1200.0 600.0))

(fn `GetRemainingAmmo`
  (returns (ReturnValue :type Integer))
  (switch `EAmmoType` (`TP_WeaponComponent.AmmoType` (`self.CurrentWeapon`))
    (:`None`
      (return 999))
    (:`Primary`
      (return 999))
    (:`Special`
      (return 999))
    (:`Heavy`
      (return 999))))

(fn `GetTraceForward`
  (returns (ReturnValue :type "Vector Structure"))
  (return (`KismetMathLibrary.GetForwardVector` (`Controller.GetControlRotation` (`self.GetController`)))))

(fn `GetTraceStart`
  (returns (ReturnValue :type "Vector Structure"))
  (return (`self.K2_GetActorLocation`)))

(fn `GetWielderControlRotation`
  (returns (ReturnValue :type "Rotator Structure"))
  (return (`self.K2_GetActorRotation` (`self.GetController`))))

(fn `InstantDetachWeapon`
  (returns (ReturnValue :type Boolean))
  (return false))

(fn `ReserveAttackToken`
  (params (Amount :type Integer))
  (returns (Success :type Boolean))
  (bind _success (`/Game/DamageSystem/AC_DamageSystem.ReservAttackToken` (`self.BPC_DamageSystem`) Amount))
  (return _success))

(fn `SetRemainingAmmo`
  (params (newValue :type Integer))
  (returns (ReturnValue :type Integer))
  (switch `EAmmoType` (`TP_WeaponComponent.AmmoType` (`self.CurrentWeapon`))
    (:`None`
      (return 999))
    (:`Primary`
      (return 999))
    (:`Special`
      (return 999))
    (:`Heavy`
      (return 999))))

(fn `UpdateMovementSpeed`
  (params (SpeedType :type "/Game/Enemies/AI/Enums/E_MovementSpeed Enum" :default "NewEnumerator0"))
  (returns (`Speed Value` :type "Float (double-precision)"))
  (set `CharacterMovementComponent.MaxWalkSpeed` (select `/Game/Enemies/AI/Enums/E_MovementSpeed` SpeedType :`NewEnumerator1` 200.0 :`NewEnumerator2` 600.0 :`NewEnumerator3` 750.0 :!type "Float (single-precision)") (`self.CharacterMovement`))
  (return 0.0))

(fn `UserConstructionScript`
  (`parent.UserConstructionScript`))