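; Base weapon Blueprint that turns WeaponComponent equip, stow and fire events into damage, sounds and effects.
; Hitscan hits apply damage with a crit multiplier, report it and feed lazily spawned, attached FX, decal, impact and sound actors.
; Projectile fire spawns a CustomProjectile aimed from the muzzle, whose impact applies damage, optionally spawning an AOE splash at reduced damage.
; Melee hit scans only play weapon sound here.
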(event `self.WeaponComponent.OnStowDelegate`
  (params (WeaponWielder :type "Actor Object Reference") (Weapon :type "TP_WeaponComponent Object Reference"))
  (message `WeaponWielderInterface.OnStow` WeaponWielder)
  (`self.SetInUse` false))

(event `self.WeaponComponent.OnEquipDelegate`
  (params (WeaponWielder :type "Actor Object Reference") (Weapon :type "TP_WeaponComponent Object Reference"))
  (message `WeaponWielderInterface.OnEquip` WeaponWielder))

(event `self.SetInUse`
  (params (InUse :type Boolean))
  (`parent.SetInUse` InUse)
  (if InUse
    (bind _aspawn (cast `Pawn` (`self.GetOwner`)))
    (message `WeaponWielderInterface.AttachWeapon` _aspawn (`self.WeaponComponent`))))

(event `self.WeaponComponent.OnMeleeWeaponHitScanDelegate`
  (params (HitResults :type "Array of HitResult Structure"))
  (`self.PlayMeleeSound` HitResults))

(event `self.WeaponComponent.OnWeaponHitScanFireDelegate`
  (params (HitResults :type "Array of HitResult Structure"))
  (`self.Deploy HitscanFiredFX` HitResults))

(event `self.WeaponComponent.OnWeaponProjectileFireDelegate`
  (params (HitResult :type "HitResult Structure"))
  (bind (_bblockinghit _binitialoverlap _time _distance _location _impactpoint _normal _impactnormal _physmat _hitactor _hitcomponent _hitbonename _bonename _hititem _elementindex _faceindex _tracestart _traceend) (`GameplayStatics.BreakHitResult` HitResult))
  (bind _weaponcomponent (`self.WeaponComponent`))
  (bind _returnvalue (`SceneComponent.GetSocketLocation` (`self.WeaponComponent`) (`self.MuzzleSocket`)))
  (bind _returnvalue_2 (`TP_WeaponComponent.GetOwningWeaponWielder` _weaponcomponent))
  (`self.DeployProjectileFiredFX` HitResult)
  (bind _returnvalue_3 (`|SpawnActorFromClass` (`self.CustomProjectile`) (`KismetMathLibrary.MakeTransform` _returnvalue (`KismetMathLibrary.FindLookAtRotation` _returnvalue (select `bool` _bblockinghit :`false` _traceend :`true` _location))) "Undefined" "MultiplyWithRoot" _returnvalue_2 (`TP_WeaponComponent.ProjectileSpeed` _weaponcomponent) 0.0 (`TP_WeaponComponent.ShouldHomig` _weaponcomponent) (`TP_WeaponComponent.HomingAccelerance` _weaponcomponent) true null _returnvalue_2))
  (bind _asprimitive_component (cast `PrimitiveComponent` (`Actor.RootComponent` (`TP_WeaponComponent.GetOwningWeaponWielder` (`self.WeaponComponent`)))))
  (`PrimitiveComponent.IgnoreActorWhenMoving` _asprimitive_component _returnvalue_3 true)
  (add `CustomProjectile.OnProjectileImpactDelegate` _returnvalue_3 (delegate `ProjectileImpact`)))

(event `ProjectileImpact`
  (params (OtherActor :type "Actor Object Reference") (Hit :type "HitResult Structure"))
  (bind (_bblockinghit _binitialoverlap _time _distance _location _impactpoint _normal _impactnormal _physmat _hitactor _hitcomponent _hitbonename) (`GameplayStatics.BreakHitResult` Hit))
  (bind _aoeclass (`self.AOEClass`))
  (bind _returnvalue (`TP_WeaponComponent.GetOwningWeaponWielder` (`self.WeaponComponent`)))
  (if (`KismetSystemLibrary.IsValidClass` _aoeclass)
    (bind _returnvalue_2 (`|SpawnActorFromClass` _aoeclass (`KismetMathLibrary.MakeTransform` _location) "Undefined" "MultiplyWithRoot" null (`TP_WeaponComponent.GetOwningWeaponWielder` (`self.WeaponComponent`))))
    (bind _asbp_aoe_projectile_splash_base (cast `/Game/DamageSystem/AOE/Splash/BP_AOE_Projectile_Splash_Base` _returnvalue_2))
    (bind _output_get (set `/Game/DamageSystem/AOE/Splash/BP_AOE_Projectile_Splash_Base.SplashDamage` (* (`TP_WeaponComponent.Damage` (`self.WeaponComponent`)) 0.65) _asbp_aoe_projectile_splash_base))
    (`/Game/DamageSystem/AOE/BP_AOE_Base.Trigger` _asbp_aoe_projectile_splash_base OtherActor))
  (bind (_wasdamaged _wasdamagedtodeath _finaldamage _iscriticalhit) (message `/Game/DamageSystem/BPI_Damagable.TakeDamage` OtherActor (make `/Game/DamageSystem/Struct/S_DamageInfo` _output_get "NewEnumerator2" "NewEnumerator1" false false true false _location _normal _hitbonename 1.0) (`TP_WeaponComponent.GetOwningWeaponWielder` (`self.WeaponComponent`)) _location 0.0))
  (if _wasdamaged
    (`AISense_Damage.ReportDamageEvent` OtherActor _returnvalue _finaldamage (`self.K2_GetActorLocation` (`TP_WeaponComponent.GetOwningWeaponWielder` (`self.WeaponComponent`))))
    (message `/Game/DamageSystem/BPI_Damagable.DamageDealt` _returnvalue _wasdamagedtodeath _iscriticalhit _location _finaldamage)))

(fn `Deploy HitscanFiredFX`
  (params (`Hit Result` :type "Array of HitResult Structure"))
  (locals (MeleeWeaponFired :type Boolean :default false))
  (bind _weaponcomponent (`self.WeaponComponent`))
  (bind _weaponcomponent_2 (`self.WeaponComponent`))
  (bind _impactsufacetypes (`self.ImpactSufaceTypes`))
  (bind _returnvalue (`TP_WeaponComponent.GetOwningWeaponWielder` (`self.WeaponComponent`)))
  (`|ExecutionSequence`
    (:`then_0`
      (`KismetArrayLibrary.Array_Clear` (`self.ImpactPositions`))
      (`KismetArrayLibrary.Array_Clear` (`self.ImpactNormals`))
      (`KismetArrayLibrary.Array_Clear` (`self.ImpactSufaceTypes`))
      (`KismetArrayLibrary.Array_Clear` (`self.TracerPositions`))
      (for _array_element `Hit Result`
        (bind (_bblockinghit _binitialoverlap _time _distance _location _impactpoint _normal _impactnormal _physmat _hitactor _hitcomponent _hitbonename _bonename _hititem _elementindex _faceindex _tracestart _traceend) (`GameplayStatics.BreakHitResult` _array_element))
        (`KismetArrayLibrary.Array_Add` (`self.TracerPositions`) _location)
        (`KismetArrayLibrary.Array_Add` (`self.ImpactPositions`) _location)
        (`KismetArrayLibrary.Array_Add` (`self.ImpactNormals`) _normal)
        (`/Engine/EditorBlueprintResources/StandardMacros.IsValid` _physmat
          (:`Is Valid`
            (`KismetArrayLibrary.Array_Add` _impactsufacetypes (`PhysicalMaterial.SurfaceType` _physmat)))
          (:`Is Not Valid`
            (`KismetArrayLibrary.Array_Add` _impactsufacetypes "SurfaceType_Default")))
        (bind (_wasdamaged _wasdamagedtodeath _finaldamage _iscriticalhit) (message `/Game/DamageSystem/BPI_Damagable.TakeDamage` _hitactor (make `/Game/DamageSystem/Struct/S_DamageInfo` (`TP_WeaponComponent.Damage` (`self.WeaponComponent`)) "NewEnumerator2" "NewEnumerator1" false false false false _location _normal _hitbonename 1.75) (`TP_WeaponComponent.GetOwningWeaponWielder` (`self.WeaponComponent`)) (0.0 0.0 0.0) 0.0))
        (if _wasdamaged
          (`AISense_Damage.ReportDamageEvent` _hitactor _returnvalue _finaldamage (`self.K2_GetActorLocation` _returnvalue))
          (message `/Game/DamageSystem/BPI_Damagable.DamageDealt` (`TP_WeaponComponent.GetOwningWeaponWielder` (`self.WeaponComponent`)) _wasdamagedtodeath _iscriticalhit _location _finaldamage)))
      (set `self.MuzzlePosition` (`SceneComponent.GetSocketLocation` (`self.WeaponComponent`) (`self.MuzzleSocket`))))
    (:`then_1`
      (`/Engine/EditorBlueprintResources/StandardMacros.IsValid` (`self.BP_WeaponFX`)
        (:`Is Valid`
          _)
        (:`Is Not Valid`
          (bind _returnvalue_2 (`|SpawnActorFromClass` "/Game/DamageSystem/Weapons/default/Effects/BP_WeaponFX.BP_WeaponFX_C" (`KismetMathLibrary.MakeTransform` (0.0 0.0 0.0)) "Undefined" "MultiplyWithRoot" null (`self.MuzzleFlashFX`) null (`self.TracerFX`) (`self.ShellEjectMesh`) (`self.Muzzle Socket`) (`self.Shell Eject Socket`) (`self.WeaponComponent`) null))
          (bind _output_get (set `self.BP_WeaponFX` _returnvalue_2))
          (`self.K2_AttachToComponent` _output_get (`self.WeaponComponent`) "None" "KeepRelative" "KeepRelative" "KeepRelative" true)))
      (`/Game/DamageSystem/Weapons/default/Effects/BP_WeaponFX.WeaponFired` (`self.BP_WeaponFX`) (`self.TracerPositions`)))
    (:`then_2`
      (`/Engine/EditorBlueprintResources/StandardMacros.IsValid` (`self.BP_WeaponDecalsFX`)
        (:`Is Valid`
          _)
        (:`Is Not Valid`
          (bind _returnvalue_3 (`|SpawnActorFromClass` "/Game/DamageSystem/Weapons/default/Effects/BP_WeaponDecals.BP_WeaponDecals_C" (`KismetMathLibrary.MakeTransform` (0.0 0.0 0.0)) "Undefined" "MultiplyWithRoot" null null))
          (bind _output_get_2 (set `self.BP_WeaponDecalsFX` _returnvalue_3))
          (`self.K2_AttachToComponent` _output_get_2 (`self.WeaponComponent`) "None" "KeepRelative" "KeepRelative" "KeepRelative" true)))
      (`/Game/DamageSystem/Weapons/default/Effects/BP_WeaponDecals.WeaponFired` (`self.BP_WeaponDecalsFX`) (`self.ImpactPositions`) (`self.ImpactNormals`) (`self.ImpactSufaceTypes`) (`self.MuzzlePosition`)))
    (:`then_3`
      (if (`KismetArrayLibrary.Array_IsNotEmpty` (`self.ImpactPositions`))
        (`/Engine/EditorBlueprintResources/StandardMacros.IsValid` (`self.BP_WeaponImpactsFX`)
          (:`Is Valid`
            _)
          (:`Is Not Valid`
            (bind _returnvalue_4 (`|SpawnActorFromClass` "/Game/DamageSystem/Weapons/default/Effects/BP_WeaponImpacts.BP_WeaponImpacts_C" (`KismetMathLibrary.MakeTransform` (0.0 0.0 0.0)) "Undefined" "MultiplyWithRoot" null null))
            (bind _output_get_3 (set `self.BP_WeaponImpactsFX` _returnvalue_4))
            (`self.K2_AttachToComponent` _output_get_3 (`self.WeaponComponent`) "None" "KeepRelative" "KeepRelative" "KeepRelative" true)))
        (`/Game/DamageSystem/Weapons/default/Effects/BP_WeaponImpacts.WeaponFired` (`self.BP_WeaponImpactsFX`) (`self.ImpactPositions`) (`self.ImpactNormals`) (`self.ImpactSufaceTypes`) (`self.MuzzlePosition`))))
    (:`then_4`
      (if (not (`TP_WeaponComponent.IsMeleeWeapon` (`self.WeaponComponent`)))
        (`/Engine/EditorBlueprintResources/StandardMacros.IsValid` (`self.BP_WeaponSounds`)
          (:`Is Valid`
            _)
          (:`Is Not Valid`
            (bind _returnvalue_5 (`|SpawnActorFromClass` "/Game/DamageSystem/Weapons/default/Effects/BP_WeaponSounds.BP_WeaponSounds_C" (`KismetMathLibrary.MakeTransform` (0.0 0.0 0.0)) "Undefined" "MultiplyWithRoot" null (`self.WeaponComponent`) (`TP_WeaponComponent.FireDelay` _weaponcomponent) (`TP_WeaponComponent.FireSound` _weaponcomponent) null))
            (bind _output_get_4 (set `self.BP_WeaponSounds` _returnvalue_5))
            (`self.K2_AttachToComponent` _output_get_4 _weaponcomponent_2 "None" "KeepRelative" "KeepRelative" "KeepRelative" true)))
        (`/Game/DamageSystem/Weapons/default/Effects/BP_WeaponSounds.WeaponFired` (`self.BP_WeaponSounds`) _weaponcomponent_2)))
    (:`then_5`
      (return))))

(fn `DeployProjectileFiredFX`
  (params (`Hit Result` :type "HitResult Structure"))
  (bind _weaponcomponent (`self.WeaponComponent`))
  (bind (_returnvalue_location _returnvalue_rotation) (`KismetMathLibrary.BreakTransform` (`SceneComponent.GetSocketTransform` _weaponcomponent (`self.MuzzleSocket`) "RTS_Component")))
  (bind _returnvalue_location_2 (`KismetMathLibrary.BreakTransform` (`SceneComponent.GetSocketTransform` _weaponcomponent (`self.MuzzleSocket`) "RTS_World")))
  (bind _returnvalue (`GameplayStatics.SpawnSoundAtLocation` (`TP_WeaponComponent.FireSound` _weaponcomponent) (`SceneComponent.GetSocketLocation` _weaponcomponent (`self.MuzzleSocket`)) (struct) 1.0 1.0 0.0 null null))
  (`AudioParameterControllerInterface.SetFloatParameter` _returnvalue "ShotInterval" (`TP_WeaponComponent.FireDelay` _weaponcomponent))
  (`AudioParameterControllerInterface.SetTriggerParameter` _returnvalue "Fire")
  (bind _returnvalue_2 (`NiagaraFunctionLibrary.SpawnSystemAttached` (`self.MuzzleFlashFX`) (`self.DefaultSceneRoot`) "None" _returnvalue_location _returnvalue_rotation "KeepRelativeOffset" true))
  (`NiagaraComponent.SetVariableVec3` _returnvalue_2 "User.Direction" (`KismetMathLibrary.Normal` (- (`|GetArrayItem` (`self.ImpactPositions`)) _returnvalue_location_2)))
  (`NiagaraComponent.SetVariableBool` _returnvalue_2 "User.Trigger" true))

(fn `PlayMeleeSound`
  (params (`Hit Result` :type "Array of HitResult Structure"))
  (locals (MeleeWeaponFired :type Boolean :default false))
  (bind _weaponcomponent (`self.WeaponComponent`))
  (bind _weaponcomponent_2 (`self.WeaponComponent`))
  (`|ExecutionSequence`
    (:`then_0`
      (`/Engine/EditorBlueprintResources/StandardMacros.IsValid` (`self.BP_WeaponSounds`)
        (:`Is Valid`
          _)
        (:`Is Not Valid`
          (bind _returnvalue (`|SpawnActorFromClass` "/Game/DamageSystem/Weapons/default/Effects/BP_WeaponSounds.BP_WeaponSounds_C" (`KismetMathLibrary.MakeTransform` (0.0 0.0 0.0)) "Undefined" "MultiplyWithRoot" null (`self.WeaponComponent`) (`TP_WeaponComponent.FireDelay` _weaponcomponent) (`TP_WeaponComponent.FireSound` _weaponcomponent) null))
          (bind _output_get (set `self.BP_WeaponSounds` _returnvalue))
          (`self.K2_AttachToComponent` _output_get _weaponcomponent_2 "None" "KeepRelative" "KeepRelative" "KeepRelative" true)))
      (`/Game/DamageSystem/Weapons/default/Effects/BP_WeaponSounds.WeaponFired` (`self.BP_WeaponSounds`) _weaponcomponent_2))
    (:`then_5`
      (return))))

(fn `UserConstructionScript`
  (`parent.UserConstructionScript`))