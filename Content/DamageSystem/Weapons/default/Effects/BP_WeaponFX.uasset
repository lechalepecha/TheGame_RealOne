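; Weapon effects actor that plays Niagara muzzle flash, shell eject and tracer effects when WeaponFired is called.
; Each system spawns from a weapon mesh socket transform only when missing or inactive, then gets retriggered by flipping its User.Trigger bool.
; The first impact position sets the flash direction and feeds the tracer's position array.
; A retriggerable delay loop destroys the actor once all three systems are invalid.
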(event `WeaponFired`
  (params (ImpactPositions :type "Array of Vector Structure"))
  (bind _ns_muzzleflash (`self.NS_MuzzleFlash`))
  (bind _ns_shelleject (`self.NS_ShellEject`))
  (bind _ns_tracer (`self.NS_Tracer`))
  (bind (_returnvalue_location _returnvalue_rotation) (`KismetMathLibrary.BreakTransform` (`SceneComponent.GetSocketTransform` (`self.WeaponMesh`) (`self.ShellEjectSocket`) "RTS_Component")))
  (bind (_returnvalue_location_2 _returnvalue_rotation_2) (`KismetMathLibrary.BreakTransform` (`SceneComponent.GetSocketTransform` (`self.WeaponMesh`) (`self.MuzzleSocket`) "RTS_Component")))
  (bind (_returnvalue_location_3 _returnvalue_rotation_3) (`KismetMathLibrary.BreakTransform` (`SceneComponent.GetSocketTransform` (`self.WeaponMesh`) (`self.MuzzleSocket`) "RTS_Component")))
  (bind _returnvalue_location_4 (`KismetMathLibrary.BreakTransform` (`SceneComponent.GetSocketTransform` (`self.WeaponMesh`) (`self.MuzzleSocket`) "RTS_World")))
  (set `self.ImpactPositions` ImpactPositions)
  (`|ExecutionSequence`
    (:`then_0`
      (`self.MuzzleFlashFX`
        (:`then`
          (`/Engine/EditorBlueprintResources/StandardMacros.IsValid` _ns_muzzleflash
            (:`Is Valid`
              (if (not (`ActorComponent.IsActive` _ns_muzzleflash))
                (bind _returnvalue (`NiagaraFunctionLibrary.SpawnSystemAtLocation` (`self.MuzzleFlashFX`) _returnvalue_location_2 _returnvalue_rotation_2 :!label _label))
                (set `self.NS_MuzzleFlash` _returnvalue)
                (set `self.MuzzleFlashTrigger` false)))
            (:`Is Not Valid`
              (goto _label)))
          (set `self.MuzzleFlashTrigger` (not (`self.MuzzleFlashTrigger`)))
          (`NiagaraComponent.SetVariableVec3` (`self.NS_MuzzleFlash`) "User.Direction" (`KismetMathLibrary.Normal` (- (`|GetArrayItem` (`self.ImpactPositions`)) _returnvalue_location_4)))
          (`NiagaraComponent.SetVariableBool` (`self.NS_MuzzleFlash`) "User.Trigger" (`self.MuzzleFlashTrigger`)))
        (:`else`)))
    (:`then_1`
      (`self.ShellEjectFX`
        (:`then`
          (`/Engine/EditorBlueprintResources/StandardMacros.IsValid` _ns_shelleject
            (:`Is Valid`
              (if (not (`ActorComponent.IsActive` _ns_shelleject))
                (bind _returnvalue_2 (`NiagaraFunctionLibrary.SpawnSystemAttached` (`self.ShellEjectFX`) (`self.DefaultSceneRoot`) "None" _returnvalue_location _returnvalue_rotation "KeepRelativeOffset" true :!label _label_2))
                (set `self.NS_ShellEject` _returnvalue_2)
                (`NiagaraComponent.SetVariableStaticMesh` (`self.NS_ShellEject`) "User.ShellEjectStaticMesh" (`self.ShellEjectMesh`))
                (set `self.ShellEjectTrigger` false)))
            (:`Is Not Valid`
              (goto _label_2)))
          (set `self.ShellEjectTrigger` (not (`self.ShellEjectTrigger`)))
          (`NiagaraComponent.SetVariableBool` (`self.NS_ShellEject`) "User.Trigger" (`self.ShellEjectTrigger`)))
        (:`else`)))
    (:`then_2`
      (`self.TracerFX`
        (:`then`
          (`/Engine/EditorBlueprintResources/StandardMacros.IsValid` _ns_tracer
            (:`Is Valid`
              (if (not (`ActorComponent.IsActive` _ns_tracer))
                (bind _returnvalue_3 (`NiagaraFunctionLibrary.SpawnSystemAttached` (`self.TracerFX`) (`self.DefaultSceneRoot`) "None" _returnvalue_location_3 _returnvalue_rotation_3 "KeepRelativeOffset" true :!label _label_3))
                (set `self.NS_Tracer` _returnvalue_3)
                (set `self.TracerTrigger` false)))
            (:`Is Not Valid`
              (goto _label_3)))
          (set `self.TracerTrigger` (not (`self.TracerTrigger`)))
          (`NiagaraComponent.SetVariableBool` (`self.NS_Tracer`) "User.Trigger" (`self.TracerTrigger`))
          (`NiagaraDataInterfaceArrayFunctionLibrary.SetNiagaraArrayVector` (`self.NS_Tracer`) "User.ImpactPositions" (`|MakeArray` (`|GetArrayItem` (`self.ImpactPositions`)))))
        (:`else`)))
    (:`then_3`
      (`KismetSystemLibrary.RetriggerableDelay` 0.3 :!label _label_4)
      (if (or (`KismetSystemLibrary.IsValid` (`self.NS_MuzzleFlash`)) (`KismetSystemLibrary.IsValid` (`self.NS_ShellEject`)) (`KismetSystemLibrary.IsValid` (`self.NS_Tracer`)))
        (goto _label_4)
        (else
          (`self.K2_DestroyActor`))))))

(fn `UserConstructionScript`)