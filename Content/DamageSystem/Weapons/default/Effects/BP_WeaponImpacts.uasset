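; Weapon impact actor that plays surface-specific Niagara effects and sounds when WeaponFired supplies hit positions, normals and surfaces.
; SplitArrayBySurface buckets hits into Concrete, Glass, Body and Default, though concrete normals land in the positions array.
; Concrete and Glass each batch hits into one reusable Niagara system through User array parameters, while Body and Default spawn per hit.
; A retriggerable delay destroys the actor once both batched systems are inactive.
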(event `WeaponFired`
  (params (ImpactPosiotions :type "Array of Vector Structure") (ImpactNormals :type "Array of Vector Structure") (ImpactSurfaces :type "Array of EPhysicalSurface Enum") (MuzzlePosition :type "Vector Structure"))
  (bind _ns_concrete (`self.NS_Concrete`))
  (bind _ns_glass (`self.NS_Glass`))
  (bind _output (`|GetArrayItem` (`self.GlassImpacts`)))
  (bind _output_2 (`|GetArrayItem` (`self.ConcnreteImpacts`)))
  (set `self.Impact Posiotions` ImpactPosiotions)
  (set `self.Impact Normals` ImpactNormals)
  (set `self.Impact Surfaces` ImpactSurfaces)
  (set `self.Muzzle Position` MuzzlePosition)
  (`self.SplitArrayBySurface`)
  (`|ExecutionSequence`
    (:`then_0`
      (if (`KismetArrayLibrary.Array_IsNotEmpty` (`self.ConcnreteImpacts`))
        (`/Engine/EditorBlueprintResources/StandardMacros.IsValid` _ns_concrete
          (:`Is Valid`
            (if (`ActorComponent.IsActive` _ns_concrete)
              (`SceneComponent.K2_SetWorldLocation` (`self.NS_Concrete`) _output_2 false false)
              (else
                (bind _returnvalue (`NiagaraFunctionLibrary.SpawnSystemAtLocation` null (`|GetArrayItem` (`self.ConcnreteImpacts`)) :!label _label))
                (set `self.NS_Concrete` _returnvalue))))
          (:`Is Not Valid`
            (goto _label)))
        (`NiagaraDataInterfaceArrayFunctionLibrary.SetNiagaraArrayPosition` (`self.NS_Concrete`) "User.ImpactPositions" (`self.ConcnreteImpacts`))
        (`NiagaraDataInterfaceArrayFunctionLibrary.SetNiagaraArrayVector` (`self.NS_Concrete`) "User.ImpactNormals" (`self.ConcreteNormals`))
        (`NiagaraComponent.SetVariableInt` (`self.NS_Concrete`) "User.NumberOfHits" (`KismetArrayLibrary.Array_Length` (`self.ConcnreteImpacts`)))
        (`NiagaraComponent.SetVariablePosition` (`self.NS_Concrete`) "User.MuzzlePosition" (`self.Muzzle Position`))
        (`ActorComponent.Activate` (`self.NS_Concrete`) false)
        (`GameplayStatics.SpawnSoundAtLocation` null _output_2 (struct) 1.0 1.0 0.0 null null)))
    (:`then_1`
      (if (`KismetArrayLibrary.Array_IsNotEmpty` (`self.GlassImpacts`))
        (`/Engine/EditorBlueprintResources/StandardMacros.IsValid` _ns_glass
          (:`Is Valid`
            (if (`ActorComponent.IsActive` _ns_glass)
              (`SceneComponent.K2_SetWorldLocation` (`self.NS_Glass`) _output false false)
              (else
                (bind _returnvalue_2 (`NiagaraFunctionLibrary.SpawnSystemAtLocation` null (`|GetArrayItem` (`self.GlassImpacts`)) :!label _label_2))
                (set `self.NS_Glass` _returnvalue_2))))
          (:`Is Not Valid`
            (goto _label_2)))
        (`NiagaraDataInterfaceArrayFunctionLibrary.SetNiagaraArrayPosition` (`self.NS_Glass`) "User.ImpactPositions" (`self.GlassImpacts`))
        (`NiagaraDataInterfaceArrayFunctionLibrary.SetNiagaraArrayVector` (`self.NS_Glass`) "User.ImpactNormals" (`self.GlassNormals`))
        (`NiagaraComponent.SetVariableInt` (`self.NS_Glass`) "User.NumberOfHits" (`KismetArrayLibrary.Array_Length` (`self.GlassImpacts`)))
        (`NiagaraComponent.SetVariablePosition` (`self.NS_Glass`) "User.MuzzlePosition" (`self.Muzzle Position`))
        (`ActorComponent.Activate` (`self.NS_Glass`) false)
        (`GameplayStatics.SpawnSoundAtLocation` null _output (struct) 1.0 1.0 0.0 null null)))
    (:`then_2`
      (if (`KismetArrayLibrary.Array_IsNotEmpty` (`self.BodyImpacts`))
        (for (_array_element _array_index) (`self.BodyImpacts`)
          (`NiagaraFunctionLibrary.SpawnSystemAtLocation` null _array_element (`KismetMathLibrary.Conv_VectorToRotator` (`|GetArrayItem` (`self.BodyNormals`) _array_index)))
          (`GameplayStatics.SpawnSoundAtLocation` null _array_element (struct) 1.0 1.0 0.0 null null))))
    (:`then_3`
      (if (`KismetArrayLibrary.Array_IsNotEmpty` (`self.DefaultImpacts`))
        (for (_array_element_2 _array_index_2) (`self.DefaultImpacts`)
          (`NiagaraFunctionLibrary.SpawnSystemAtLocation` null _array_element_2 (`KismetMathLibrary.Conv_VectorToRotator` (`|GetArrayItem` (`self.DefaultNormals`) _array_index_2)))
          (`GameplayStatics.SpawnSoundAtLocation` null _array_element_2 (struct) 1.0 1.0 0.0 null null))))
    (:`then_4`
      (`KismetArrayLibrary.Array_Clear` (`self.GlassNormals`))
      (`KismetArrayLibrary.Array_Clear` (`self.GlassImpacts`))
      (`KismetArrayLibrary.Array_Clear` (`self.ConcreteNormals`))
      (`KismetArrayLibrary.Array_Clear` (`self.ConcnreteImpacts`))
      (`KismetArrayLibrary.Array_Clear` (`self.BodyNormals`))
      (`KismetArrayLibrary.Array_Clear` (`self.BodyImpacts`))
      (`KismetArrayLibrary.Array_Clear` (`self.DefaultNormals`))
      (`KismetArrayLibrary.Array_Clear` (`self.DefaultImpacts`)))
    (:`then_5`
      (`KismetSystemLibrary.RetriggerableDelay` 3.0 :!label _label_3)
      (if (or (`ActorComponent.IsActive` (`self.NS_Concrete`)) (`ActorComponent.IsActive` (`self.NS_Glass`)))
        (goto _label_3)
        (else
          (`self.K2_DestroyActor`))))))

(fn `SplitArrayBySurface`
  (for (_array_element _array_index) (`self.Impact Surfaces`)
    (switch `EPhysicalSurface` _array_element
      (:`SurfaceType_Default`
        (`KismetArrayLibrary.Array_Add` (`self.DefaultImpacts`) (`|GetArrayItem` (`self.Impact Posiotions`) _array_index))
        (`KismetArrayLibrary.Array_Add` (`self.DefaultNormals`) (`|GetArrayItem` (`self.Impact Normals`) _array_index)))
      (:`SurfaceType1`
        (`KismetArrayLibrary.Array_Add` (`self.BodyImpacts`) (`|GetArrayItem` (`self.Impact Posiotions`) _array_index))
        (`KismetArrayLibrary.Array_Add` (`self.BodyNormals`) (`|GetArrayItem` (`self.Impact Normals`) _array_index)))
      (:`SurfaceType2`
        (`KismetArrayLibrary.Array_Add` (`self.ConcnreteImpacts`) (`|GetArrayItem` (`self.Impact Posiotions`) _array_index))
        (`KismetArrayLibrary.Array_Add` (`self.ConcnreteImpacts`) (`|GetArrayItem` (`self.Impact Normals`) _array_index)))
      (:`SurfaceType3`
        (`KismetArrayLibrary.Array_Add` (`self.GlassImpacts`) (`|GetArrayItem` (`self.Impact Posiotions`) _array_index))
        (`KismetArrayLibrary.Array_Add` (`self.GlassNormals`) (`|GetArrayItem` (`self.Impact Normals`) _array_index))))))

(fn `UserConstructionScript`)