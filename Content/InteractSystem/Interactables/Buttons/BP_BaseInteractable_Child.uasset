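; Child Blueprint of an interactable base, filed under Buttons, that plays a sound when the first-person character interacts with it.
; Interact casts the interactor to BP_FPCharacter and, if the button is pressed, plays CompileFailed_Cue at the actor's location, then clears the character's pressed flag.
; The sphere overlap event is empty, the default events are disabled, and construction only calls the parent.
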(event `/Game/InteractSystem/BPI_Interactable.Interact`
  (params (Interactor :type "Actor Object Reference") (IsInteractButtonPressed :type Boolean))
  (bind _asbp_fpcharacter (cast `/Game/FirstPerson/Blueprints/BP_FPCharacter` Interactor))
  (if IsInteractButtonPressed
    (`GameplayStatics.PlaySoundAtLocation` "/Engine/EditorSounds/Notifications/CompileFailed_Cue.CompileFailed_Cue" (`self.K2_GetActorLocation`) (struct) 1.0 1.0 0.0 null null null null)
    (set `/Game/FirstPerson/Blueprints/BP_FPCharacter.IsInteractButtonPressed` false _asbp_fpcharacter)))

(event `self.Sphere.OnComponentBeginOverlap`
  (params (OverlappedComponent :type "PrimitiveComponent Object Reference") (OtherActor :type "Actor Object Reference") (OtherComp :type "PrimitiveComponent Object Reference") (OtherBodyIndex :type Integer) (bFromSweep :type Boolean) (SweepResult :type "HitResult Structure (by ref)")))

(fn `UserConstructionScript`
  (`parent.UserConstructionScript`))