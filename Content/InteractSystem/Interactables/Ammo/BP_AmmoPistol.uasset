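; BP_AmmoPistol is an interactable pistol ammo pickup that adds a fixed amount of reserve ammo to the player.
; It applies an outline overlay material on BeginPlay.
; On Interact, it casts the interactor to BP_FPCharacter, raises its primary remaining ammo through a message call and refreshes the HUD ammo display.
; It then plays a pickup sound at its location and destroys itself.
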(event `self.ReceiveBeginPlay`
  (`parent.ReceiveBeginPlay`)
  (set `self.OverlayMaterial` "/Game/Materials/Outlines/MI_AmmoOutline.MI_AmmoOutline"))

(event `self.Interact`
  (params (Interactor :type "Actor Object Reference") (IsInteractButtonPressed :type Boolean))
  (bind _asbp_fpcharacter (cast `/Game/FirstPerson/Blueprints/BP_FPCharacter` Interactor))
  (message `WeaponWielderInterface.SetRemainingAmmo` _asbp_fpcharacter (+ (`MainCharacter.PrimaryAmmoRemaining` _asbp_fpcharacter) 20))
  (`/Game/HUD/WBP_FirstPersonHUD.Update Ammo UI` (`/Game/FirstPerson/Blueprints/BP_FPCharacter.PlayerHUDRef` _asbp_fpcharacter))
  (`GameplayStatics.SpawnSoundAtLocation` "/Engine/VREditor/Sounds/UI/Dockable_Window_Pick_Up.Dockable_Window_Pick_Up" (`self.K2_GetActorLocation`) (struct) 1.0 1.0 0.0 null null)
  (`self.K2_DestroyActor`))

(fn `UserConstructionScript`
  (`parent.UserConstructionScript`))