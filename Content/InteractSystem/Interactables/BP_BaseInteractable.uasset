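; BP_BaseInteractable is a base interactable actor that shows a hint when the first-person character approaches.
; An outer trigger creates an icon widget and highlights the mesh through custom depth stencil, then clears both on exit, delaying widget removal briefly.
; An inner sphere, centered on the mesh and sized from its height in the construction script, calls Interact on overlap with the button flagged as not pressed.
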(event `self.OutlineSphereTrace.OnComponentBeginOverlap`
  (params (OverlappedComponent :type "PrimitiveComponent Object Reference") (OtherActor :type "Actor Object Reference") (OtherComp :type "PrimitiveComponent Object Reference") (OtherBodyIndex :type Integer) (bFromSweep :type Boolean) (SweepResult :type "HitResult Structure (by ref)"))
  (bind _widget (`self.Widget`))
  (cast `/Game/FirstPerson/Blueprints/BP_FPCharacter` OtherActor)
  (bind _returnvalue (`|CreateWidget` "/Game/HUD/WBP_IntearctIcon.WBP_IntearctIcon_C"))
  (bind _output_get (set `self.InteractionWidget` _returnvalue))
  (`WidgetComponent.SetWidget` _widget _output_get)
  (`SceneComponent.SetVisibility` _widget true false)
  (bind _interactionwidget (`self.InteractionWidget`)
    (:`then`
      (if (not (`self.HintVisible`))
        (set `self.HintVisible` true)
        (`PrimitiveComponent.SetCustomDepthStencilValue` (`self.StaticMesh`) 1)))
    (:`else`)))

(event `self.OutlineSphereTrace.OnComponentEndOverlap`
  (params (OverlappedComponent :type "PrimitiveComponent Object Reference") (OtherActor :type "Actor Object Reference") (OtherComp :type "PrimitiveComponent Object Reference") (OtherBodyIndex :type Integer))
  (cast `/Game/FirstPerson/Blueprints/BP_FPCharacter` OtherActor)
  (bind _interactionwidget (`self.InteractionWidget`)
    (:`then`
      (if (`self.HintVisible`)
        (set `self.HintVisible` false)
        (`PrimitiveComponent.SetCustomDepthStencilValue` (`self.StaticMesh`) 0))
      (`KismetSystemLibrary.Delay` 0.2)
      (`Widget.RemoveFromParent` (`self.InteractionWidget`))
      (set `self.InteractionWidget` null)
      (`SceneComponent.SetVisibility` (`self.Widget`) false false))
    (:`else`)))

(event `self.Sphere.OnComponentBeginOverlap`
  (params (OverlappedComponent :type "PrimitiveComponent Object Reference") (OtherActor :type "Actor Object Reference") (OtherComp :type "PrimitiveComponent Object Reference") (OtherBodyIndex :type Integer) (bFromSweep :type Boolean) (SweepResult :type "HitResult Structure (by ref)"))
  (bind _asbp_fpcharacter (cast `/Game/FirstPerson/Blueprints/BP_FPCharacter` OtherActor))
  (`/Game/InteractSystem/BPI_Interactable.Interact` _asbp_fpcharacter))

(fn `UserConstructionScript`
  (bind _sphere (`self.Sphere`))
  (bind (_min _max) (`StaticMeshComponent.GetLocalBounds` (`self.StaticMesh`)))
  (bind (_returnvalue_x _returnvalue_y _returnvalue_z) (`KismetMathLibrary.BreakVector` (- _max _min)))
  (`SceneComponent.K2_SetRelativeLocation` _sphere (/ (+ _min _max) 2.0) false false)
  (`SphereComponent.SetSphereRadius` _sphere _returnvalue_z true))